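; BP_AINav_Player is the player variant of campaign fleet navigation, overriding how a fleet picks its destination.
; When the fleet has no valid DestinationObject, SetDestination assigns the player controller's ClickLocation, provided that marker is not hidden.
; It then always calls the parent SetDestination, leaving the rest of the navigation logic to the base class.
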(fn `SetDestination`
  (bind _clicklocation (`/Game/Game/BP_PlayerController.ClickLocation` (`/Game/Actors/BP_CampaignFleet.PlayerController` (`self.CampaignFleet`))))
  (`|ExecutionSequence`
    (:`then_0`
      (`/Engine/EditorBlueprintResources/StandardMacros.IsValid` (`KismetSystemLibrary.Conv_InterfaceToObject` (`/Game/Actors/BP_CampaignFleet.DestinationObject` (`self.CampaignFleet`)))
        (:`Is Not Valid`
          (if (not (`Actor.bHidden` _clicklocation))
            (set `/Game/Actors/BP_CampaignFleet.DestinationObject` _clicklocation (`self.CampaignFleet`))))))
    (:`then_1`
      (`parent.SetDestination`))))