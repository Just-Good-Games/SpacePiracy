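; AI navigation Blueprint for the tutorial pirate fleet in the campaign solar system.
; It overrides SetDestination: on one specific campaign tutorial step, it sets the fleet's destination object to the player fleet, reached through the fleet's camera pawn.
; It then always calls the parent SetDestination.
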(fn `SetDestination`
  (bind _camerapawn (`/Game/Actors/BP_CampaignFleet.CameraPawn` (`self.CampaignFleet`)))
  (`|ExecutionSequence`
    (:`then_0`
      (if (`|EnumEquality` (`/Game/ActorComponents/BP_SpaceTutorial.CurrentStep` (`/Game/Game/BP_GameMode.CampaignTutorial` (`/Game/Game/BP_HUD.Gamemode` (`/Game/ActorComponents/BP_CampaignManager.HUD` (`/Game/Actors/BP_SolarSystem.CampaignManager` (`/Game/Actors/BP_CampaignFleet.SolarSystem` (`self.CampaignFleet`))))))) "NewEnumerator5")
        (`/Engine/EditorBlueprintResources/StandardMacros.IsValid` _camerapawn
          (:`Is Valid`
            (set `/Game/Actors/BP_CampaignFleet.DestinationObject` (`/Game/Game/BP_CameraPawn.PlayerFleet` _camerapawn) (`self.CampaignFleet`))))))
    (:`then_1`
      (`parent.SetDestination`))))