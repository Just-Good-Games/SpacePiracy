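; BP_AINav_Base is a base AI navigation object that adjusts the destination of a campaign fleet.
; Setup stores the fleet it controls.
; SetDestination acts only when that fleet's destination is another campaign fleet, redirecting it to the target's SlipStream if the target has one and the controlled fleet has none.
; Otherwise, the target fleet remains the destination.
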(fn `SetDestination`
  (bind _campaignfleet (`self.CampaignFleet`))
  (bind _campaignfleet_2 (`self.CampaignFleet`))
  (`/Engine/EditorBlueprintResources/StandardMacros.IsValid` _campaignfleet_2
    (:`Is Valid`
      (bind _asbp_campaign_fleet (cast `/Game/Actors/BP_CampaignFleet` (`/Game/Actors/BP_CampaignFleet.DestinationObject` _campaignfleet_2)))
      (bind _slipstream (`/Game/Actors/BP_CampaignFleet.SlipStream` _asbp_campaign_fleet))
      (`/Engine/EditorBlueprintResources/StandardMacros.IsValid` _slipstream
        (:`Is Valid`
          (`/Engine/EditorBlueprintResources/StandardMacros.IsValid` (`/Game/Actors/BP_CampaignFleet.SlipStream` (`self.CampaignFleet`))
            (:`Is Valid`
              (set `/Game/Actors/BP_CampaignFleet.DestinationObject` _asbp_campaign_fleet _campaignfleet :!label _label))
            (:`Is Not Valid`
              (set `/Game/Actors/BP_CampaignFleet.DestinationObject` _slipstream _campaignfleet))))
        (:`Is Not Valid`
          (goto _label))))))

(fn `Setup`
  (params (CampaignFleet :type "/Game/Actors/BP_CampaignFleet Object Reference"))
  (set `self.CampaignFleet` CampaignFleet))