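; BP_Battle runs a turn-based battle between attacking and defending fleets, opening the combat UI for player battles and queueing others in GameMode.
; Each turn pairs ships round-robin; a maneuver roll winner picks the strategy, with retreat allowed once the opposing side has cycled.
; Damage rolls capture or destroy ships, recording bounties for kills; captures, destruction and damage finalize when a side empties.
; Roll logs are kept only for player battles.
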(fn `AddLogLine`
  (params (LogLine :type String))
  (switch `/Game/GlobalEnums/E_BattleType` (`self.BattleType`)
    (:`NewEnumerator2`
      _)
    (:`NewEnumerator3`
      _))
  (`KismetArrayLibrary.Array_Add` (`self.Logs`) LogLine))

(fn `AddLogLineForShip`
  (params (Ship :type "/Game/Objects/BP_Ship Object Reference") (LogLine :type String))
  (switch `/Game/GlobalEnums/E_BattleType` (`self.BattleType`)
    (:`NewEnumerator2`
      _)
    (:`NewEnumerator3`
      _))
  (`self.AddLogLine` (`KismetStringLibrary.Concat_StrStr` (`/Game/Objects/BP_Ship.ShipName` Ship) " - " LogLine)))

(fn `DefeatCurrentShip`
  (params (bAttacker :type Boolean) (bCaptured :type Boolean))
  (bind _bcaptured (`local.bCaptured`))
  (bind _currentattackingship (`self.CurrentAttackingShip`))
  (bind _currentdefendingship (`self.CurrentDefendingShip`))
  (`self.RemoveCurrentShip` bAttacker)
  (if bAttacker
    (if _bcaptured
      (`/Game/ActorComponents/BP_Fleet.TemporaryCaptureShip` (`/Game/Objects/BP_Ship.Fleet` (`self.CurrentDefendingShip`)) (`self.CurrentAttackingShip`))
      (else
        (`KismetArrayLibrary.Array_Add` (`self.DestroyedShips`) (`self.CurrentAttackingShip`))
        (`/Game/ActorComponents/BP_Fleet.RecordCrimeCommitted` (`/Game/Objects/BP_Ship.Fleet` (`self.CurrentDefendingShip`)) (`/Game/ActorComponents/BP_Fleet.Faction` (`/Game/Objects/BP_Ship.Fleet` _currentattackingship)) "NewEnumerator3" (* (`/Game/Objects/BP_Ship.GetShipStat` _currentattackingship "NewEnumerator2") 1000))))
    (elif _bcaptured
      (`/Game/ActorComponents/BP_Fleet.TemporaryCaptureShip` (`/Game/Objects/BP_Ship.Fleet` (`self.CurrentAttackingShip`)) (`self.CurrentDefendingShip`))
      (else
        (`KismetArrayLibrary.Array_Add` (`self.DestroyedShips`) (`self.CurrentDefendingShip`))
        (`/Game/ActorComponents/BP_Fleet.RecordCrimeCommitted` (`/Game/Objects/BP_Ship.Fleet` (`self.CurrentAttackingShip`)) (`/Game/ActorComponents/BP_Fleet.Faction` (`/Game/Objects/BP_Ship.Fleet` _currentdefendingship)) "NewEnumerator3" (* (`/Game/Objects/BP_Ship.GetShipStat` _currentdefendingship "NewEnumerator2") 1000))))))

(fn `FinalizeShipCaptures`
  (for _array_element (`self.AttackingFleets`)
    (`/Engine/EditorBlueprintResources/StandardMacros.IsValid` _array_element
      (:`Is Valid`
        (`/Game/ActorComponents/BP_Fleet.FinalizeShipCaptures` _array_element (> (`KismetArrayLibrary.Array_Length` (`self.AttackingShips`)) 0)))))
  (for _array_element_2 (`self.DefendingFleets`)
    (`/Engine/EditorBlueprintResources/StandardMacros.IsValid` _array_element_2
      (:`Is Valid`
        (`/Game/ActorComponents/BP_Fleet.FinalizeShipCaptures` _array_element_2 (> (`KismetArrayLibrary.Array_Length` (`self.DefendingShips`)) 0))))))

(fn `FinalizeShipDamage`
  (for _array_element (`self.AttackingFleets`)
    (`/Engine/EditorBlueprintResources/StandardMacros.IsValid` _array_element
      (:`Is Valid`
        (for _array_element_2 (`/Game/ActorComponents/BP_Fleet.Ships` _array_element)
          (`/Game/Objects/BP_Ship.ApplyPostBattleDamage` _array_element_2)))))
  (for _array_element_3 (`self.DefendingFleets`)
    (`/Engine/EditorBlueprintResources/StandardMacros.IsValid` _array_element_3
      (:`Is Valid`
        (for _array_element_4 (`/Game/ActorComponents/BP_Fleet.Ships` _array_element_3)
          (`/Game/Objects/BP_Ship.ApplyPostBattleDamage` _array_element_4))))))

(fn `FinalizeShipsDestroyed`
  (for _array_element (`self.DestroyedShips`)
    (`/Game/Objects/BP_Ship.DestroyShip` _array_element)))

(fn `FleetsToShips`
  (params (bAttacking :type Boolean))
  (bind _returnvalue (select `bool` bAttacking :`false` (`self.DefendingShips`) :`true` (`self.AttackingShips`)))
  (`KismetArrayLibrary.Array_Clear` _returnvalue)
  (for _array_element (select `bool` bAttacking :`false` (`self.DefendingFleets`) :`true` (`self.AttackingFleets`))
    (bind _ships (`/Game/ActorComponents/BP_Fleet.Ships` _array_element))
    (`KismetArrayLibrary.Array_Append` _returnvalue _ships)
    (`|ExecutionSequence`
      (:`then_0`
        (if (`/Game/ActorComponents/BP_Fleet.bIsPlayer` _array_element)
          (set `self.BattleType` (select `bool` (`local.bAttacking`) :`false` "NewEnumerator3" :`true` "NewEnumerator2" :!type "/Game/GlobalEnums/E_BattleType Enum"))))
      (:`then_1`
        (for _array_element_2 _ships
          (`/Game/Objects/BP_Ship.CalculateBattleStats` _array_element_2))))))

(fn `GetCurrentAttackingShip`
  (returns (Ship :type "/Game/Objects/BP_Ship Object Reference"))
  (return (`self.CurrentAttackingShip`)))

(fn `GetCurrentDefendingShip`
  (returns (Ship :type "/Game/Objects/BP_Ship Object Reference"))
  (return (`self.CurrentDefendingShip`)))

(fn `GetCurrentShip`
  (params (bIsAttacker :type Boolean))
  (returns (Ship :type "/Game/Objects/BP_Ship Object Reference"))
  (if bIsAttacker
    (return (`self.CurrentAttackingShip`))
    (else
      (return (`self.CurrentDefendingShip`)))))

(fn `GetCurrentShipBattleState`
  (params (bIsAttacker :type Boolean))
  (returns (BattleShipState :type "/Game/GlobalEnums/E_BattleShipState Enum"))
  (locals (bHasAdvantage :type Boolean))
  (bind _bhasadvantage (`local.bHasAdvantage`))
  (set `local.bHasAdvantage` (select `/Game/GlobalEnums/E_ManeuverAdvantage` (`self.CurrentManeuverAdvantage`) :`NewEnumerator1` bIsAttacker :`NewEnumerator2` (not bIsAttacker)))
  (switch `/Game/GlobalEnums/E_BattleStrategy` (`self.CurrentStrategy`)
    (:`NewEnumerator0`
      (return "NewEnumerator1"))
    (:`NewEnumerator1`
      (if _bhasadvantage
        (return "NewEnumerator1")
        (else
          (return "NewEnumerator2"))))
    (:`NewEnumerator2`
      (if _bhasadvantage
        (return "NewEnumerator3")
        (else
          (return "NewEnumerator1"))))))

(fn `GetIsPlayerTurn`
  (returns (Return :type Boolean))
  (return (or (`/Game/ActorComponents/BP_Fleet.bIsPlayer` (`/Game/Objects/BP_Ship.Fleet` (`self.CurrentAttackingShip`))) (`/Game/ActorComponents/BP_Fleet.bIsPlayer` (`/Game/Objects/BP_Ship.Fleet` (`self.CurrentDefendingShip`))))))

(fn `InitializeTurn`
  (returns (bBattleOver :type Boolean))
  (`|ExecutionSequence`
    (:`then_0`
      (if (not (and (> (`KismetArrayLibrary.Array_Length` (`self.AttackingShips`)) 0) (> (`KismetArrayLibrary.Array_Length` (`self.DefendingShips`)) 0)))
        (`self.FinalizeShipCaptures`)
        (`self.FinalizeShipsDestroyed`)
        (`self.FinalizeShipDamage`)
        (`|ExecutionSequence`
          (:`then_0`
            (if (`self.bCampaignBattle`)
              (`/Game/Game/BP_GameMode.SetPauseState` (`self.GameMode`) false)
              (else
                (`Widget.SetVisibility` (`/Game/Game/BP_HUD.MainMenuUI` (`self.Hud`)) "Visible"))))
          (:`then_1`
            (`self.FinishedBattle`)
            (return true)))))
    (:`then_1`
      (bind _result (`/Engine/EditorBlueprintResources/StandardMacros.IncrementInt` (`self.CurrentAttackerIndex`))
        (:`  `
          (if (>= _result (`KismetArrayLibrary.Array_Length` (`self.AttackingShips`)))
            (set `self.CurrentAttackerIndex` 0)
            (set `self.bDefenderCanRetreat` true)))))
    (:`then_2`
      (bind _result_2 (`/Engine/EditorBlueprintResources/StandardMacros.IncrementInt` (`self.CurrentDefenderIndex`))
        (:`  `
          (if (>= _result_2 (`KismetArrayLibrary.Array_Length` (`self.DefendingShips`)))
            (set `self.CurrentDefenderIndex` 0)
            (set `self.bAttackerCanRetreat` true)))))
    (:`then_3`
      (set `self.CurrentAttackingShip` (`|GetArrayItem` (`self.AttackingShips`) (`self.CurrentAttackerIndex`)))
      (set `self.CurrentDefendingShip` (`|GetArrayItem` (`self.DefendingShips`) (`self.CurrentDefenderIndex`)))
      (`/Game/Objects/BP_Ship.SetupPreviewPhase` (`self.CurrentAttackingShip`))
      (`/Game/Objects/BP_Ship.SetupPreviewPhase` (`self.CurrentDefendingShip`)))
    (:`then_4`
      (set `self.CurrentStrategy` "NewEnumerator0")
      (set `self.CurrentManeuverAdvantage` "NewEnumerator0"))
    (:`then_5`
      (return false))))

(fn `LogDamageRolls`
  (bind _currentattackingship (`self.CurrentAttackingShip`))
  (bind _currentdefendingship (`self.CurrentDefendingShip`))
  (switch `/Game/GlobalEnums/E_BattleType` (`self.BattleType`)
    (:`NewEnumerator2`
      _)
    (:`NewEnumerator3`
      _))
  (`|ExecutionSequence`
    (:`then_0`
      (`self.LogRoll` _currentattackingship "NewEnumerator3")
      (switch `/Game/GlobalEnums/E_ManeuverAdvantage` (`self.CurrentManeuverAdvantage`)
        (:`NewEnumerator1`
          (`self.LogRoll` _currentattackingship "NewEnumerator5"))))
    (:`then_1`
      (`self.LogRoll` (`self.CurrentDefendingShip`) "NewEnumerator2")
      (`self.LogDamageTaken` (`self.CurrentDefendingShip`) (`self.CurrentAttackingShip`))
      (`self.AddLogLine` ""))
    (:`then_2`
      (`self.LogRoll` _currentdefendingship "NewEnumerator3")
      (switch `/Game/GlobalEnums/E_ManeuverAdvantage` (`self.CurrentManeuverAdvantage`)
        (:`NewEnumerator2`
          (`self.LogRoll` _currentdefendingship "NewEnumerator5"))))
    (:`then_3`
      (`self.LogRoll` (`self.CurrentAttackingShip`) "NewEnumerator2")
      (`self.LogDamageTaken` (`self.CurrentAttackingShip`) (`self.CurrentDefendingShip`)))))

(fn `LogDamageTaken`
  (params (DamagedShip :type "/Game/Objects/BP_Ship Object Reference") (DamagingShip :type "/Game/Objects/BP_Ship Object Reference"))
  (bind _damagingship (`local.DamagingShip`))
  (`self.AddLogLineForShip` DamagedShip (`KismetStringLibrary.Concat_StrStr` "Took " (`KismetStringLibrary.Conv_IntToString` (`KismetMathLibrary.Max` (- (+ (`/Game/Objects/BP_Ship.GetBattleRoll` _damagingship "NewEnumerator3") (`/Game/Objects/BP_Ship.GetBattleRoll` _damagingship "NewEnumerator5")) (`/Game/Objects/BP_Ship.GetBattleRoll` (`local.DamagedShip`) "NewEnumerator2")))) " Damage.")))

(fn `LogManeuverRolls`
  (switch `/Game/GlobalEnums/E_BattleType` (`self.BattleType`)
    (:`NewEnumerator2`
      _)
    (:`NewEnumerator3`
      _))
  (`self.AddLogLine` " \n[Maneuver Phase]")
  (`self.LogRoll` (`self.CurrentAttackingShip`) "NewEnumerator1")
  (`self.LogRoll` (`self.CurrentDefendingShip`) "NewEnumerator1"))

(fn `LogRoll`
  (params (Ship :type "/Game/Objects/BP_Ship Object Reference") (Stat :type "/Game/GlobalEnums/E_BattleTarget Enum" :default "NewEnumerator0"))
  (bind _stat (`local.Stat`))
  (bind _ship (`local.Ship`))
  (bind _gamemode (`self.GameMode`))
  (bind _value (`/Game/Objects/BP_Ship.GetBattleStat` _ship _stat))
  (bind _balternatezerocalculation (`/Game/Objects/BP_Ship.GetBattleStatAlternateZeroCalc` _ship _stat))
  (`self.AddLogLineForShip` Ship (`KismetStringLibrary.Concat_StrStr` (`|GetEnumeratorNameAsString` (`local.Stat`)) " Roll [" (`KismetStringLibrary.Conv_IntToString` (`/Game/Game/BP_GameMode.MinimumRoll` _gamemode _value _balternatezerocalculation)) ", " (`KismetStringLibrary.Conv_IntToString` (`/Game/Game/BP_GameMode.MaximumRoll` _gamemode _value _balternatezerocalculation)) "] -> " (`KismetStringLibrary.Conv_IntToString` (`/Game/Objects/BP_Ship.GetBattleRoll` (`local.Ship`) _stat)))))

(fn `RemoveCurrentShip`
  (params (bAttacker :type Boolean))
  (if bAttacker
    (`KismetArrayLibrary.Array_RemoveItem` (`self.AttackingShips`) (`self.CurrentAttackingShip`))
    (`/Engine/EditorBlueprintResources/StandardMacros.DecrementInt` (`self.CurrentAttackerIndex`))
    (else
      (`KismetArrayLibrary.Array_RemoveItem` (`self.DefendingShips`) (`self.CurrentDefendingShip`))
      (`/Engine/EditorBlueprintResources/StandardMacros.DecrementInt` (`self.CurrentDefenderIndex`)))))

(fn `ResolveDamage`
  (locals (AttackingDamage :type Integer) (DefendingDamage :type Integer) (bAttackerDestroyed :type Boolean) (bDefenderDestroyed :type Boolean) (bAttackerCaptured :type Boolean) (bDefenderCaptured :type Boolean))
  (bind _currentdefendingship (`self.CurrentDefendingShip`))
  (bind _currentattackingship (`self.CurrentAttackingShip`))
  (bind _currentattackingship_2 (`self.CurrentAttackingShip`))
  (bind _currentattackingship_3 (`self.CurrentAttackingShip`))
  (bind _currentdefendingship_2 (`self.CurrentDefendingShip`))
  (bind _currentdefendingship_3 (`self.CurrentDefendingShip`))
  (bind _returnvalue (select `bool` (`|EnumEquality` (`self.CurrentManeuverAdvantage`) "NewEnumerator1") :`false` (`self.CurrentDefendingShip`) :`true` (`self.CurrentAttackingShip`)))
  (`|ExecutionSequence`
    (:`then_0`
      (`self.AddLogLine` " \n[Damage Phase]")
      (switch `/Game/GlobalEnums/E_BattleStrategy` (`self.CurrentStrategy`)
        (:`NewEnumerator1`
          (`/Game/Objects/BP_Ship.RollDamagePhase` (`self.CurrentAttackingShip`))
          (`/Game/Objects/BP_Ship.RollDamagePhase` (`self.CurrentDefendingShip`))
          (`self.LogDamageRolls`)
          (`|ExecutionSequence`
            (:`then_0`
              (bind _result (`/Game/Objects/BP_Ship.ApplyBattleDamage` (`self.CurrentDefendingShip`) (`/Game/Objects/BP_Ship.GetBattleTarget` (`self.CurrentAttackingShip`)) (- (+ (`/Game/Objects/BP_Ship.GetBattleRoll` _currentattackingship "NewEnumerator3") (`/Game/Objects/BP_Ship.GetBattleRoll` _currentattackingship "NewEnumerator5")) (`/Game/Objects/BP_Ship.GetBattleRoll` (`self.CurrentDefendingShip`) "NewEnumerator2"))))
              (switch `/Game/GlobalEnums/E_BattleResult` _result
                (:`NewEnumerator2`
                  (`self.DefeatCurrentShip` false true)
                  (set `local.bDefenderCaptured` true)
                  (`/Game/Objects/BP_Ship.SetBattleShipState` _currentdefendingship_2 "NewEnumerator5")
                  (`self.AddLogLineForShip` _currentdefendingship_3 "Was captured."))
                (:`NewEnumerator3`
                  (`self.DefeatCurrentShip` false)
                  (set `local.bDefenderDestroyed` true)
                  (`/Game/Objects/BP_Ship.SetBattleShipState` _currentdefendingship_2 "NewEnumerator4")
                  (`self.AddLogLineForShip` _currentdefendingship_3 "Was destroyed."))))
            (:`then_1`
              (bind _result_2 (`/Game/Objects/BP_Ship.ApplyBattleDamage` (`self.CurrentAttackingShip`) (`/Game/Objects/BP_Ship.GetBattleTarget` (`self.CurrentDefendingShip`)) (- (+ (`/Game/Objects/BP_Ship.GetBattleRoll` _currentdefendingship "NewEnumerator3") (`/Game/Objects/BP_Ship.GetBattleRoll` _currentdefendingship "NewEnumerator5")) (`/Game/Objects/BP_Ship.GetBattleRoll` (`self.CurrentAttackingShip`) "NewEnumerator2"))))
              (switch `/Game/GlobalEnums/E_BattleResult` _result_2
                (:`NewEnumerator2`
                  (`self.DefeatCurrentShip` true true)
                  (set `local.bAttackerCaptured` true)
                  (`/Game/Objects/BP_Ship.SetBattleShipState` _currentattackingship_2 "NewEnumerator5")
                  (`self.AddLogLineForShip` _currentattackingship_3 "Was captured."))
                (:`NewEnumerator3`
                  (`self.DefeatCurrentShip` true)
                  (set `local.bAttackerDestroyed` true)
                  (`/Game/Objects/BP_Ship.SetBattleShipState` _currentattackingship_2 "NewEnumerator4")
                  (`self.AddLogLineForShip` _currentattackingship_3 "Was destroyed."))))))
        (:`NewEnumerator2`
          (`self.RemoveCurrentShip` (`|EnumEquality` (`self.CurrentManeuverAdvantage`) "NewEnumerator1"))
          (`/Game/Objects/BP_Ship.SetBattleShipState` _returnvalue "NewEnumerator3")
          (`self.AddLogLineForShip` _returnvalue "Fled"))))
    (:`then_1`
      (`self.TurnEnd`))))

(fn `ResolveManeuver`
  (locals (AttackingManeuver :type Integer :default 0) (DefendingManeuver :type Integer :default 0))
  (bind _currentattackingship (`self.CurrentAttackingShip`))
  (`/Game/Objects/BP_Ship.RollManeuverPhase` (`self.CurrentAttackingShip`))
  (`/Game/Objects/BP_Ship.RollManeuverPhase` (`self.CurrentDefendingShip`))
  (`self.LogManeuverRolls`)
  (set `local.AttackingManeuver` (`/Game/Objects/BP_Ship.GetBattleRoll` (`self.CurrentAttackingShip`) "NewEnumerator1"))
  (set `local.DefendingManeuver` (`/Game/Objects/BP_Ship.GetBattleRoll` (`self.CurrentDefendingShip`) "NewEnumerator1"))
  (if (> (`local.AttackingManeuver`) (`local.DefendingManeuver`))
    (set `self.CurrentManeuverAdvantage` "NewEnumerator1")
    (`/Game/Objects/BP_Ship.SetBattleShipState` (`self.CurrentDefendingShip`) "NewEnumerator2")
    (set `self.CurrentStrategy` (`/Game/Objects/BP_Ship.GetBattleStrategy` (`self.CurrentAttackingShip`) (`self.bAttackerCanRetreat`)))
    (`self.AddLogLineForShip` (`self.CurrentAttackingShip`) "Has the maneuver advantage.")
    (elif (< (`local.AttackingManeuver`) (`local.DefendingManeuver`))
      (set `self.CurrentManeuverAdvantage` "NewEnumerator2")
      (`/Game/Objects/BP_Ship.SetBattleShipState` _currentattackingship "NewEnumerator2")
      (set `self.CurrentStrategy` (`/Game/Objects/BP_Ship.GetBattleStrategy` (`self.CurrentDefendingShip`) (`self.bDefenderCanRetreat`)))
      (`self.AddLogLineForShip` (`self.CurrentDefendingShip`) "Has the maneuver advantage.")
      (else
        (set `self.CurrentManeuverAdvantage` "NewEnumerator0")
        (`/Game/Objects/BP_Ship.SetBattleShipState` _currentattackingship "NewEnumerator2")
        (`/Game/Objects/BP_Ship.SetBattleShipState` (`self.CurrentDefendingShip`) "NewEnumerator2")
        (set `self.CurrentStrategy` "NewEnumerator1")
        (`self.AddLogLine` "Neither ship out maneuvered the other."))))
  (return))

(fn `ResolveTurn`
  (returns (bBattleOver :type Boolean))
  (bind _bbattleover (`self.InitializeTurn`))
  (if _bbattleover
    (return true)
    (else
      (`self.ResolveManeuver`)
      (`self.ResolveDamage`)
      (return false))))

(fn `StartBattle`
  (set `self.BattleType` "NewEnumerator1")
  (`self.FleetsToShips` true)
  (`self.FleetsToShips` false)
  (switch `/Game/GlobalEnums/E_BattleType` (`self.BattleType`)
    (:`NewEnumerator1`
      (`/Game/Game/BP_GameMode.QueueBattle` (`self.GameMode`) self))
    (:`NewEnumerator2`
      (`/Game/Game/BP_GameMode.SetPauseState` (`self.GameMode`) true :!label _label)
      (`/Game/Widgets/Battle/WB_BattleUI.StartBattle` (`/Game/Game/BP_HUD.CombatUI` (`self.Hud`)) (`|EnumEquality` (`self.BattleType`) "NewEnumerator2") self))
    (:`NewEnumerator3`
      (goto _label))))