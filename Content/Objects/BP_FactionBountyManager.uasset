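; Faction bounty manager that keeps campaign fleets ordered by their bounty with one faction and assigns each a rank and alert level.
; Inserts use a recursive binary search in ascending order, while SortBounties gnome-sorts in descending order; both prune invalid fleets.
; Inserts, removals and sorts reapply ranks from array index.
; Alert level scales index by half a hardcoded faction's planet count, or is 3 when that count is zero.
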(fn `ClearBounties`
  (`KismetArrayLibrary.Array_Clear` (`self.CampaignFleets`)))

(fn `FindInsertIndex`
  (params (NewFleetBounty :type Integer) (StartIndex :type Integer) (EndIndex :type Integer))
  (returns (InsertIndex :type Integer))
  (locals (TestIndex :type Integer) (TestCampaignFleet :type "/Game/Actors/BP_CampaignFleet Object Reference") (TestBounty :type Integer))
  (if (== StartIndex EndIndex)
    (return (`local.StartIndex`))
    (else
      (bind _output_get (set `local.TestIndex` (/ (+ (`local.StartIndex`) (`local.EndIndex`)) 2)))
      (bind _output_get_2 (set `local.TestCampaignFleet` (`|GetArrayItem` (`self.CampaignFleets`) _output_get)))
      (`/Engine/EditorBlueprintResources/StandardMacros.IsValid` _output_get_2
        (:`Is Valid`
          (bind _output_get_3 (set `local.TestBounty` (`/Game/ActorComponents/BP_Fleet.GetFactionBountyAmount` (`/Game/Actors/BP_CampaignFleet.FleetComponent` (`local.TestCampaignFleet`)) (`self.Faction`))))
          (`/JGGErrorAndTesting/Macros/BM_Comparison.BranchCompare` (`local.NewFleetBounty`) _output_get_3
            (:`Less`
              (bind _insertindex (`self.FindInsertIndex` (`local.NewFleetBounty`) (`local.StartIndex`) (`local.TestIndex`)))
              (return _insertindex))
            (:`Equal`
              (return (+ (`local.TestIndex`) 1)))
            (:`Greater`
              (bind _insertindex_2 (`self.FindInsertIndex` (`local.NewFleetBounty`) (+ (`local.TestIndex`) 1) (`local.EndIndex`)))
              (return _insertindex_2))))
        (:`Is Not Valid`
          (`KismetArrayLibrary.Array_Remove` (`self.CampaignFleets`) (`local.TestIndex`))
          (bind _insertindex_3 (`self.FindInsertIndex` (`local.NewFleetBounty`) (`local.StartIndex`) (- (`local.EndIndex`) 1)))
          (return _insertindex_3))))))

(fn `InsertNewFleet`
  (params (CampaignFleet :type "/Game/Actors/BP_CampaignFleet Object Reference"))
  (locals (InsertIndex :type Integer :default 0))
  (bind _insertindex (`self.FindInsertIndex` (`/Game/ActorComponents/BP_Fleet.GetFactionBountyAmount` (`/Game/Actors/BP_CampaignFleet.FleetComponent` CampaignFleet) (`self.Faction`)) 0 (`KismetArrayLibrary.Array_Length` (`self.CampaignFleets`))))
  (bind _output_get (set `local.InsertIndex` _insertindex))
  (`KismetArrayLibrary.Array_Insert` (`self.CampaignFleets`) (`local.CampaignFleet`) _output_get)
  (`self.ReapplyRanksAndAlerts`))

(fn `ReapplyRanksAndAlerts`
  (if (!= (`/Game/ActorComponents/BP_CampaignManager.GetNumPlanetsOfFaction` (`self.CampaignManager`) "NewEnumerator0") 0)
    (for (_array_element _array_index) (`self.CampaignFleets`)
      (`/Game/ActorComponents/BP_Fleet.SetAlertAndRank` (`/Game/Actors/BP_CampaignFleet.FleetComponent` _array_element) (`self.Faction`) _array_index (`KismetMathLibrary.FTrunc` (* _array_index (/ (`/Game/ActorComponents/BP_CampaignManager.GetNumPlanetsOfFaction` (`self.CampaignManager`) "NewEnumerator0") 2.0)))))
    (else
      (for (_array_element_2 _array_index_2) (`self.CampaignFleets`)
        (`/Game/ActorComponents/BP_Fleet.SetAlertAndRank` (`/Game/Actors/BP_CampaignFleet.FleetComponent` _array_element_2) (`self.Faction`) _array_index_2 3)))))

(fn `RemoveFleet`
  (params (CampaignFleet :type "/Game/Actors/BP_CampaignFleet Object Reference"))
  (locals (InsertIndex :type Integer :default 0))
  (`KismetArrayLibrary.Array_RemoveItem` (`self.CampaignFleets`) CampaignFleet)
  (`self.ReapplyRanksAndAlerts`))

(fn `SortBounties`
  (locals (Index :type Integer :default 0))
  (bind _index (`local.Index`))
  (if (< _index (- (`KismetArrayLibrary.Array_Length` (`self.CampaignFleets`)) 1)) :!label _label
    (bind _nextiterationindex (`self.SortBountiesIteration` _index))
    (set `local.Index` _nextiterationindex)
    (goto _label)
    (else
      (`self.ReapplyRanksAndAlerts`))))

(fn `SortBountiesIteration`
  (params (CurrentIndex :type Integer))
  (returns (NextIterationIndex :type Integer))
  (locals (CurrentFleet :type "/Game/Actors/BP_CampaignFleet Object Reference") (NextFleet :type "/Game/Actors/BP_CampaignFleet Object Reference") (NextIndex :type Integer))
  (set `local.NextIndex` (+ CurrentIndex 1))
  (bind _output_get (set `local.CurrentFleet` (`|GetArrayItem` (`self.CampaignFleets`) (`local.CurrentIndex`))))
  (`/Engine/EditorBlueprintResources/StandardMacros.IsValid` _output_get
    (:`Is Valid`
      (bind _output_get_2 (set `local.NextFleet` (`|GetArrayItem` (`self.CampaignFleets`) (`local.NextIndex`))))
      (`/Engine/EditorBlueprintResources/StandardMacros.IsValid` _output_get_2
        (:`Is Valid`
          (if (> (`/Game/ActorComponents/BP_Fleet.GetFactionBountyAmount` (`/Game/Actors/BP_CampaignFleet.FleetComponent` (`local.NextFleet`)) (`self.Faction`)) (`/Game/ActorComponents/BP_Fleet.GetFactionBountyAmount` (`/Game/Actors/BP_CampaignFleet.FleetComponent` (`local.CurrentFleet`)) (`self.Faction`)))
            (`KismetArrayLibrary.Array_Set` (`self.CampaignFleets`) (`local.CurrentIndex`) (`local.NextFleet`))
            (`KismetArrayLibrary.Array_Set` (`self.CampaignFleets`) (`local.NextIndex`) (`local.CurrentFleet`))
            (return (`KismetMathLibrary.Abs_Int` (- (`local.CurrentIndex`) 1)))
            (else
              (return (`local.NextIndex`)))))
        (:`Is Not Valid`
          (`KismetArrayLibrary.Array_RemoveItem` (`self.CampaignFleets`) (`local.NextFleet`))
          (return (`local.CurrentIndex`)))))
    (:`Is Not Valid`
      (`KismetArrayLibrary.Array_RemoveItem` (`self.CampaignFleets`) (`local.CurrentFleet`))
      (return (`local.CurrentIndex`)))))