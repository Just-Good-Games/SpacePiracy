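; BP_AINav_TutorialMerchant is the AI navigation Blueprint for merchant fleets in the campaign tutorial.
; It overrides SetDestination: when the fleet has no valid destination object, it picks a random entry from the tutorial's AIDestinations list, if that list is not empty.
; It then always calls the parent SetDestination to handle the rest.
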(fn `SetDestination`
  (bind _aidestinations (`/Game/ActorComponents/BP_SpaceTutorial.AIDestinations` (`/Game/Game/BP_GameMode.CampaignTutorial` (`/Game/Game/BP_HUD.Gamemode` (`/Game/ActorComponents/BP_CampaignManager.HUD` (`/Game/Actors/BP_SolarSystem.CampaignManager` (`/Game/Actors/BP_CampaignFleet.SolarSystem` (`self.CampaignFleet`))))))))
  (`|ExecutionSequence`
    (:`then_0`
      (`/Engine/EditorBlueprintResources/StandardMacros.IsValid` (`KismetSystemLibrary.Conv_InterfaceToObject` (`/Game/Actors/BP_CampaignFleet.DestinationObject` (`self.CampaignFleet`)))
        (:`Is Not Valid`
          (if (not (`KismetArrayLibrary.Array_IsEmpty` _aidestinations))
            (set `/Game/Actors/BP_CampaignFleet.DestinationObject` (`KismetArrayLibrary.Array_Random` _aidestinations) (`self.CampaignFleet`))))))
    (:`then_1`
      (`parent.SetDestination`))))