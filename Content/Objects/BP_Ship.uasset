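; A ship in a fleet, built from a template row, with deployed, destroyed and stored components that drive its stats and the fleet totals.
; Component changes check cargo or armour slots and, unless overridden, power before updating the stat maps.
; Battle stats derive from ship stats and feed phased rolls; damage cascades through systems in target-priority order, then converts into destroyed components.
; Player ships take target and strategy from the combat UI, computer ships from fleet type and faction.
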(fn `ApplyBattleDamage`
  (params (Target :type "/Game/GlobalEnums/E_BattleTarget Enum" :default "NewEnumerator0") (Damage :type Integer))
  (returns (Result :type "/Game/GlobalEnums/E_BattleResult Enum"))
  (locals (EngineFocusTargetOrder :type "Array of /Game/GlobalEnums/E_BattleTarget Enum") (ShieldFocusTargetOrder :type "Array of /Game/GlobalEnums/E_BattleTarget Enum") (GunFocusTargetOrder :type "Array of /Game/GlobalEnums/E_BattleTarget Enum") (KillFocusTargetOrder :type "Array of /Game/GlobalEnums/E_BattleTarget Enum") (CurrentDamage :type Integer))
  (bind _output_get (set `local.CurrentDamage` Damage))
  (if (> _output_get 0)
    (for _array_element (select `/Game/GlobalEnums/E_BattleTarget` Target :`NewEnumerator1` (`local.EngineFocusTargetOrder`) :`NewEnumerator2` (`local.ShieldFocusTargetOrder`) :`NewEnumerator3` (`local.GunFocusTargetOrder`) :`NewEnumerator4` (`local.KillFocusTargetOrder`))
      (bind (_remainingdamage _bdamagecontinues) (`self.ApplyBattleDamageToSystem` _array_element (`local.CurrentDamage`)))
      (set `local.CurrentDamage` _remainingdamage)
      (if (not _bdamagecontinues)
        (return "NewEnumerator1")))
    (return (select `/Game/GlobalEnums/E_BattleTarget` (`local.Target`) :`NewEnumerator0` "NewEnumerator0" :`NewEnumerator1` "NewEnumerator2" :`NewEnumerator2` "NewEnumerator2" :`NewEnumerator3` "NewEnumerator2" :`NewEnumerator4` "NewEnumerator3" :`NewEnumerator5` "NewEnumerator0" :!type "/Game/GlobalEnums/E_BattleResult Enum"))
    (else
      (return "NewEnumerator1"))))

(fn `ApplyBattleDamageToSystem`
  (params (BattleTarget :type "/Game/GlobalEnums/E_BattleTarget Enum" :default "NewEnumerator0") (Damage :type Integer))
  (returns (RemainingDamage :type Integer) (bDamageContinues :type Boolean))
  (locals (NewValue :type Integer) (ExtraDamage :type Integer) (DamageToTarget :type Integer))
  (bind _output_get (set `local.DamageToTarget` (`KismetMathLibrary.Min` (`local.Damage`) (`self.GetBattleStat` (`local.BattleTarget`)))))
  (`/JGGUniversalFunctionsAndMacros/Macros/BM_Maps.IncrementIntegerMap` (`self.BattleDamage`) (`local.BattleTarget`) _output_get
    (:`OutExec`
      (`/JGGUniversalFunctionsAndMacros/Macros/BM_Maps.IncrementIntegerMap` (`self.BattleStats`) (`local.BattleTarget`) (* (`local.DamageToTarget`) -1)
        (:`OutExec`
          (return (- (`local.Damage`) (`local.DamageToTarget`)) (== (`self.GetBattleStat` (`local.BattleTarget`)) 0)))))))

(fn `ApplyPostBattleDamage`
  (`self.CalculateStatChangeFromDamage`)
  (`self.DestroyComponentsFromStatChange`))

(fn `CalculateBattleStats`
  (bind _battlestats (`self.BattleStats`))
  (`BlueprintMapLibrary.Map_Clear` _battlestats)
  (`BlueprintMapLibrary.Map_Add` _battlestats "NewEnumerator1" (`KismetMathLibrary.FCeil` (/ (`KismetMathLibrary.Conv_IntToDouble` (`self.GetShipStat` "NewEnumerator9")) (`KismetMathLibrary.Conv_IntToDouble` (`self.GetShipStat` "NewEnumerator1")))))
  (`BlueprintMapLibrary.Map_Add` _battlestats "NewEnumerator2" (`self.GetShipStat` "NewEnumerator8"))
  (`BlueprintMapLibrary.Map_Add` _battlestats "NewEnumerator3" (`self.GetShipStat` "NewEnumerator7"))
  (`BlueprintMapLibrary.Map_Add` _battlestats "NewEnumerator5" (`self.GetShipStat` "NewEnumerator6"))
  (`BlueprintMapLibrary.Map_Add` _battlestats "NewEnumerator4" (`KismetMathLibrary.FCeil` (/ (`KismetMathLibrary.Conv_IntToDouble` (`self.GetShipStat` "NewEnumerator10")) (`KismetMathLibrary.Conv_IntToDouble` (`self.GetShipStat` "NewEnumerator3")))))
  (set `self.PreBattleStats` (`self.BattleStats`)))

(fn `CalculateStatChangeFromDamage`
  (`BlueprintMapLibrary.Map_Clear` (`self.ShipDamage`))
  (`/JGGUniversalFunctionsAndMacros/Macros/BM_Maps.IncrementIntegerMap` (`self.ShipDamage`) "NewEnumerator9" (* (`self.GetBattleDamage` "NewEnumerator1") (`self.GetShipStat` "NewEnumerator1"))
    (:`OutExec`
      (`/JGGUniversalFunctionsAndMacros/Macros/BM_Maps.IncrementIntegerMap` (`self.ShipDamage`) "NewEnumerator8" (`self.GetBattleDamage` "NewEnumerator2")
        (:`OutExec`
          (`/JGGUniversalFunctionsAndMacros/Macros/BM_Maps.IncrementIntegerMap` (`self.ShipDamage`) "NewEnumerator7" (`self.GetBattleDamage` "NewEnumerator3")
            (:`OutExec`
              (`/JGGUniversalFunctionsAndMacros/Macros/BM_Maps.IncrementIntegerMap` (`self.ShipDamage`) "NewEnumerator6" (`self.GetBattleDamage` "NewEnumerator5")
                (:`OutExec`
                  (`/JGGUniversalFunctionsAndMacros/Macros/BM_Maps.IncrementIntegerMap` (`self.ShipDamage`) "NewEnumerator10" (* (`self.GetBattleDamage` "NewEnumerator4") (`self.GetShipStat` "NewEnumerator3"))
                    (:`OutExec`
                      (`BlueprintMapLibrary.Map_Clear` (`self.BattleDamage`)))))))))))))

(fn `ChangeComponents`
  (params (ShipComponent :type "/Game/Structs/S_ShipComponent Structure") (ChangeNumber :type Integer) (State :type "/Game/GlobalEnums/E_ShipComponentState Enum" :default "NewEnumerator0") (bIgnorePowerRequirement :type Boolean :default false))
  (returns (bSuccess :type Boolean))
  (bind _changenumber (`local.ChangeNumber`))
  (bind _freearmourslots (`self.FreeArmourSlots`))
  (bind _shipcomponent (`local.ShipComponent`))
  (bind (_tradegood _rank) (break `/Game/Structs/S_ShipComponent` (`local.ShipComponent`)))
  (bind _returnvalue (select `/Game/GlobalEnums/E_ShipComponentState` State :`NewEnumerator1` (`self.DeployedComponents`) :`NewEnumerator2` (`self.DestroyedComponents`) :`NewEnumerator3` (`self.StoredComponents`)))
  (bind (_value _returnvalue_2) (`BlueprintMapLibrary.Map_Find` _returnvalue (`local.ShipComponent`)))
  (if (and (`|EnumInequality` State "NewEnumerator0") (!= ChangeNumber 0))
    (if (> (`local.ChangeNumber`) 0)
      (if (>= (select `/Game/GlobalEnums/E_TradeGoodType` (`/Game/Game/BP_GameMode.GetTradeGoodType` (`/Game/Game/BP_HUD.Gamemode` (`/Game/ActorComponents/BP_Fleet.Hud` (`self.Fleet`))) (`.TradeGood_2_520825BF4FF280580CE275961ED246F2` (break `/Game/Structs/S_ShipComponent` (`local.ShipComponent`)))) :`NewEnumerator2` (select `/Game/GlobalEnums/E_ShipComponentState` (`local.State`) :`NewEnumerator1` _freearmourslots :`NewEnumerator2` _freearmourslots :`NewEnumerator3` (`self.FreeCargoSlots`)) :`NewEnumerator3` (`self.FreeCargoSlots`)) (* (select `/Game/GlobalEnums/E_TradeGoodType` "NewEnumerator0" :`NewEnumerator2` 1 :`NewEnumerator3` (select `/Game/GlobalEnums/E_ShipComponentState` (`local.State`) :`NewEnumerator1` 2 :`NewEnumerator2` 2 :`NewEnumerator3` 1)) (`local.ChangeNumber`)))
        (if (or (>= (+ (* (`/Game/Game/BP_GameMode.GetTradeGoodProperty` (`/Game/Game/BP_HUD.Gamemode` (`/Game/ActorComponents/BP_Fleet.Hud` (`self.Fleet`))) _tradegood "NewEnumerator5" (`local.State`) _rank) (`local.ChangeNumber`)) (`self.GetShipStat` "NewEnumerator5")) 0) (`local.bIgnorePowerRequirement`))
          _
          (else
            (return false)))
        (else
          (return false)))
      (elif (and _returnvalue_2 (>= _value (* (`local.ChangeNumber`) -1)))
        _
        (else
          (return false))))
    (`/JGGUniversalFunctionsAndMacros/Macros/BM_Maps.IncrementIntegerMap` _returnvalue _shipcomponent _changenumber
      (:`OutExec`
        (`self.ChangeShipStats` _shipcomponent _changenumber (`local.State`))
        (return true)))
    (else
      (return false))))

(fn `ChangeFleet`
  (params (NewFleet :type "/Game/ActorComponents/BP_Fleet Object Reference"))
  (locals (OldFleet :type "/Game/ActorComponents/BP_Fleet Object Reference"))
  (bind _output_get (set `local.OldFleet` (`self.Fleet`)))
  (`/Game/ActorComponents/BP_Fleet.AddRemoveShip` _output_get self false)
  (`/Game/ActorComponents/BP_Fleet.AddRemoveShip` (`local.NewFleet`) self true)
  (`/Game/ActorComponents/BP_Fleet.CheckIfFleetIsDestroyed` (`local.OldFleet`)))

(fn `ChangeShipStats`
  (params (ShipComponent :type "/Game/Structs/S_ShipComponent Structure") (Change :type Integer) (State :type "/Game/GlobalEnums/E_ShipComponentState Enum" :default "NewEnumerator0"))
  (locals (StatChange :type Integer))
  (bind (_tradegood _rank) (break `/Game/Structs/S_ShipComponent` ShipComponent))
  (bind _gamemode (`/Game/Game/BP_HUD.Gamemode` (`/Game/ActorComponents/BP_Fleet.Hud` (`self.Fleet`))))
  (for _array_element (`/Game/Game/BP_GameMode.GetTradeGoodProperties` _gamemode _tradegood)
    (bind _output_get (set `local.StatChange` (* (`/Game/Game/BP_GameMode.GetTradeGoodProperty` _gamemode _tradegood _array_element (`local.State`) _rank) (`local.Change`))))
    (`/JGGUniversalFunctionsAndMacros/Macros/BM_Maps.IncrementIntegerMap` (`self.ShipStats`) _array_element _output_get
      (:`OutExec`
        (`/JGGUniversalFunctionsAndMacros/Macros/BM_Maps.IncrementIntegerMap` (`/Game/ActorComponents/BP_Fleet.FleetStats` (`self.Fleet`)) _array_element (`local.StatChange`)))))
  (switch `/Game/GlobalEnums/E_TradeGoodType` (`/Game/Game/BP_GameMode.GetTradeGoodType` (`/Game/Game/BP_HUD.Gamemode` (`/Game/ActorComponents/BP_Fleet.Hud` (`self.Fleet`))) _tradegood)
    (:`NewEnumerator1`
      (set `self.FreeCargoSlots` (`self.GetShipStat` "NewEnumerator4"))
      (set `self.FreeArmourSlots` (`self.GetShipStat` "NewEnumerator3")))
    (:`NewEnumerator2`
      (if (select `/Game/GlobalEnums/E_ShipComponentState` (`local.State`) :`NewEnumerator1` true :`NewEnumerator2` true)
        (set `self.FreeArmourSlots` (+ (* (`local.Change`) -1) (`self.FreeArmourSlots`)))
        (else
          (set `self.FreeCargoSlots` (+ (* (`local.Change`) (select `/Game/GlobalEnums/E_ShipComponentState` (`local.State`) :`NewEnumerator1` 2 :`NewEnumerator2` 2 :`NewEnumerator3` 1) -1) (`self.FreeCargoSlots`)) :!label _label))))
    (:`NewEnumerator3`
      (goto _label))))

(fn `CreateComponentsOfStateFromTemplate`
  (params (Components :type "Map of /Game/GlobalEnums/E_TradeGood Enum to Integer") (State :type "/Game/GlobalEnums/E_ShipComponentState Enum" :default "NewEnumerator0"))
  (if (`|EnumInequality` State "NewEnumerator0")
    (bind _keys (`BlueprintMapLibrary.Map_Keys` Components))
    (for _array_element _keys
      (bind (_value _returnvalue) (`BlueprintMapLibrary.Map_Find` Components _array_element))
      (if _returnvalue
        (`self.ChangeComponents` (make `/Game/Structs/S_ShipComponent` _array_element 1) _value State true)))))

(fn `CreateShipFromTemplate`
  (locals (ShipTemplateTable :type "DataTable Object Reference" :default "/Script/Engine.DataTable'/Game/DataTables/DT_ShipTemplates.DT_ShipTemplates'"))
  (bind _value (`self.GetShipStat` "NewEnumerator5"))
  (bind _returnvalue (`|GetDataTableRow` (`local.ShipTemplateTable`) (`self.ShipTemplate`))
    (:`then`
      (bind (_shiptype _deployedcomponents _destroyedcomponents _storedcomponents) (break `/Game/Structs/S_ShipTemplate` _returnvalue))
      (bind _output_get (set `self.ShipType` _shiptype))
      (`self.ChangeShipStats` (make `/Game/Structs/S_ShipComponent` _output_get 1) 1 "NewEnumerator1")
      (`self.CreateComponentsOfStateFromTemplate` _deployedcomponents "NewEnumerator1")
      (`self.CreateComponentsOfStateFromTemplate` _destroyedcomponents "NewEnumerator2")
      (`self.CreateComponentsOfStateFromTemplate` _storedcomponents "NewEnumerator3")
      (if (< _value 0)
        (`/Game/Game/BP_GameMode.PrintMessage` (`/Game/Game/BP_HUD.Gamemode` (`/Game/ActorComponents/BP_Fleet.Hud` (`self.Fleet`))) self "NewEnumerator1" (`KismetStringLibrary.Concat_StrStr` (`KismetStringLibrary.Conv_NameToString` (`self.ShipTemplate`)) " template has negative power = " (`KismetStringLibrary.Conv_IntToString` _value)) "None" false)))))

(fn `DebugPrintBattleDamage`
  (bind _keys (`BlueprintMapLibrary.Map_Keys` (`self.BattleDamage`)))
  (for _array_element _keys
    (`/Game/Game/BP_GameMode.PrintMessage` (`/Game/Game/BP_HUD.Gamemode` (`/Game/ActorComponents/BP_Fleet.Hud` (`self.Fleet`))) self "NewEnumerator0" (`KismetStringLibrary.Concat_StrStr` "BattleDamage - " (`|GetEnumeratorNameAsString` _array_element) " = " (`KismetStringLibrary.Conv_IntToString` (`self.GetBattleDamage` _array_element))) "None" false)))

(fn `DebugPrintBattleStats`
  (bind _keys (`BlueprintMapLibrary.Map_Keys` (`self.BattleStats`)))
  (for _array_element _keys
    (`/Game/Game/BP_GameMode.PrintMessage` (`/Game/Game/BP_HUD.Gamemode` (`/Game/ActorComponents/BP_Fleet.Hud` (`self.Fleet`))) self "NewEnumerator0" (`KismetStringLibrary.Concat_StrStr` "BattleStat - " (`|GetEnumeratorNameAsString` _array_element) " = " (`KismetStringLibrary.Conv_IntToString` (`self.GetBattleStat` _array_element))) "None" false)))

(fn `DebugPrintShipDamage`
  (bind _keys (`BlueprintMapLibrary.Map_Keys` (`self.ShipDamage`)))
  (for _array_element _keys
    (`/Game/Game/BP_GameMode.PrintMessage` (`/Game/Game/BP_HUD.Gamemode` (`/Game/ActorComponents/BP_Fleet.Hud` (`self.Fleet`))) self "NewEnumerator0" (`KismetStringLibrary.Concat_StrStr` "ShipDamage - " (`|GetEnumeratorNameAsString` _array_element) " = " (`KismetStringLibrary.Conv_IntToString` (`self.GetShipDamage` _array_element))) "None" false)))

(fn `DebugPrintShipStats`
  (bind _keys (`BlueprintMapLibrary.Map_Keys` (`self.ShipStats`)))
  (for _array_element _keys
    (`/Game/Game/BP_GameMode.PrintMessage` (`/Game/Game/BP_HUD.Gamemode` (`/Game/ActorComponents/BP_Fleet.Hud` (`self.Fleet`))) self "NewEnumerator0" (`KismetStringLibrary.Concat_StrStr` "ShipStat - " (`|GetEnumeratorNameAsString` _array_element) " = " (`KismetStringLibrary.Conv_IntToString` (`self.GetShipStat` _array_element))) "None" false)))

(fn `DestroyComponentsFromStatChange`
  (locals (Components :type "Array of /Game/Structs/S_ShipComponent Structure") (NumComponentsDestroyed :type Integer))
  (bind _keys (`BlueprintMapLibrary.Map_Keys` (`self.DeployedComponents`)))
  (bind _output_get (set `local.Components` _keys))
  (for _array_element _output_get
    (bind (_tradegood _rank) (break `/Game/Structs/S_ShipComponent` _array_element))
    (for _array_element_2 (`/Game/Game/BP_GameMode.GetTradeGoodProperties` (`/Game/Game/BP_HUD.Gamemode` (`/Game/ActorComponents/BP_Fleet.Hud` (`self.Fleet`))) _tradegood)
      (bind (_value _returnvalue) (`BlueprintMapLibrary.Map_Find` (`self.DeployedComponents`) _array_element))
      (if _returnvalue
        (bind _value_2 (`/Game/Game/BP_GameMode.GetTradeGoodProperty` (`/Game/Game/BP_HUD.Gamemode` (`/Game/ActorComponents/BP_Fleet.Hud` (`self.Fleet`))) _tradegood _array_element_2 "NewEnumerator1" _rank))
        (bind _output_get_2 (set `local.NumComponentsDestroyed` (`KismetMathLibrary.Min` _value (`KismetMathLibrary.Round` (`KismetMathLibrary.SafeDivide` (`KismetMathLibrary.Conv_IntToDouble` (`self.GetShipDamage` _array_element_2)) (`KismetMathLibrary.Conv_IntToDouble` _value_2))))))
        (`/JGGUniversalFunctionsAndMacros/Macros/BM_Maps.IncrementIntegerMap` (`self.ShipDamage`) _array_element_2 (* _output_get_2 _value_2 -1)
          (:`OutExec`
            (bind _bsuccess (`self.ChangeComponents` _array_element (* (`local.NumComponentsDestroyed`) -1) "NewEnumerator1"))
            (if _bsuccess
              (`self.ChangeComponents` _array_element (`local.NumComponentsDestroyed`) "NewEnumerator2")))))))
  (`BlueprintMapLibrary.Map_Clear` (`self.ShipDamage`)))

(fn `DestroyShip`
  (bind _fleet (`self.Fleet`))
  (bind _keys (`BlueprintMapLibrary.Map_Keys` (`self.ShipStats`)))
  (for _array_element _keys
    (`/JGGUniversalFunctionsAndMacros/Macros/BM_Maps.IncrementIntegerMap` (`/Game/ActorComponents/BP_Fleet.FleetStats` (`self.Fleet`)) _array_element (* (`BlueprintMapLibrary.Map_Find` (`self.ShipStats`) _array_element) -1)))
  (`KismetArrayLibrary.Array_RemoveItem` (`/Game/ActorComponents/BP_Fleet.Ships` _fleet) self)
  (`/Game/ActorComponents/BP_Fleet.CheckIfFleetIsDestroyed` _fleet))

(fn `GetBattleDamage`
  (params (Stat :type "/Game/GlobalEnums/E_BattleTarget Enum" :default "NewEnumerator0"))
  (returns (Value :type Integer))
  (bind (_value _returnvalue) (`BlueprintMapLibrary.Map_Find` (`self.BattleDamage`) Stat))
  (if _returnvalue
    (return _value)
    (else
      (return 0))))

(fn `GetBattleRoll`
  (params (Stat :type "/Game/GlobalEnums/E_BattleTarget Enum" :default "NewEnumerator0"))
  (returns (Roll :type Integer))
  (bind (_value _returnvalue) (`BlueprintMapLibrary.Map_Find` (`self.BattleRoll`) Stat))
  (if _returnvalue
    (return _value)
    (else
      (return 0))))

(fn `GetBattleStat`
  (params (Stat :type "/Game/GlobalEnums/E_BattleTarget Enum" :default "NewEnumerator0"))
  (returns (Value :type Integer))
  (bind (_value _returnvalue) (`BlueprintMapLibrary.Map_Find` (`self.BattleStats`) Stat))
  (if _returnvalue
    (return _value)
    (else
      (return 0))))

(fn `GetBattleStatAlternateZeroCalc`
  (params (Stat :type "/Game/GlobalEnums/E_BattleTarget Enum" :default "NewEnumerator0"))
  (returns (bAlternateZeroCalculation :type Boolean))
  (return (select `/Game/GlobalEnums/E_BattleTarget` Stat :`NewEnumerator1` true)))

(fn `GetBattleStatRoll`
  (params (Stat :type "/Game/GlobalEnums/E_BattleTarget Enum" :default "NewEnumerator0"))
  (returns (Value :type Integer))
  (return (`/Game/Game/BP_GameMode.RandomRoll` (`/Game/Game/BP_HUD.Gamemode` (`/Game/ActorComponents/BP_Fleet.Hud` (`self.Fleet`))) (`self.GetBattleStat` Stat) (`self.GetBattleStatAlternateZeroCalc` Stat))))

(fn `GetBattleStrategy`
  (returns (Target :type "/Game/GlobalEnums/E_BattleStrategy Enum"))
  (if (`/Game/ActorComponents/BP_Fleet.bIsPlayer` (`self.Fleet`))
    (return (`self.GetBattleStrategyPlayer`))
    (else
      (return (`self.GetBattleStrategyComputer`)))))

(fn `GetBattleStrategyComputer`
  (returns (Target :type "/Game/GlobalEnums/E_BattleStrategy Enum"))
  (return (select `/Game/GlobalEnums/E_FleetType` (`/Game/ActorComponents/BP_Fleet.FleetType` (`self.Fleet`)) :`NewEnumerator2` "NewEnumerator1" :`NewEnumerator0` "NewEnumerator1" :`NewEnumerator1` "NewEnumerator2" :`NewEnumerator3` "NewEnumerator1" :!type "/Game/GlobalEnums/E_BattleStrategy Enum")))

(fn `GetBattleStrategyPlayer`
  (returns (Strategy :type "/Game/GlobalEnums/E_BattleStrategy Enum"))
  (return (`/Game/Widgets/Battle/WB_BattleUI.PlayerStrategy` (`/Game/Game/BP_HUD.CombatUI` (`/Game/ActorComponents/BP_Fleet.Hud` (`self.Fleet`))))))

(fn `GetBattleTarget`
  (returns (Target :type "/Game/GlobalEnums/E_BattleTarget Enum"))
  (if (`/Game/ActorComponents/BP_Fleet.bIsPlayer` (`self.Fleet`))
    (return (`self.GetBattleTargetPlayer`))
    (else
      (return (`self.GetBattleTargetComputer`)))))

(fn `GetBattleTargetComputer`
  (returns (Target :type "/Game/GlobalEnums/E_BattleTarget Enum"))
  (locals (TargetOptions :type "Array of /Game/GlobalEnums/E_BattleTarget Enum"))
  (bind _fleet (`self.Fleet`))
  (bind _targetoptions (`local.TargetOptions`))
  (bind _returnvalue (select `/Game/GlobalEnums/E_Faction` (`/Game/ActorComponents/BP_Fleet.Faction` _fleet) :`NewEnumerator0` "NewEnumerator4" :`NewEnumerator5` (`|GetArrayItem` _targetoptions (`KismetMathLibrary.RandomInteger` (`KismetArrayLibrary.Array_Length` _targetoptions))) :`NewEnumerator4` "NewEnumerator4" :`NewEnumerator3` "NewEnumerator4" :`NewEnumerator2` "NewEnumerator4" :`NewEnumerator1` "NewEnumerator4"))
  (return (select `/Game/GlobalEnums/E_FleetType` (`/Game/ActorComponents/BP_Fleet.FleetType` _fleet) :`NewEnumerator2` _returnvalue :`NewEnumerator0` _returnvalue :`NewEnumerator1` "NewEnumerator1" :`NewEnumerator3` _returnvalue)))

(fn `GetBattleTargetPlayer`
  (returns (Target :type "/Game/GlobalEnums/E_BattleTarget Enum"))
  (return (`/Game/Widgets/Battle/WB_BattleUI.PlayerTarget` (`/Game/Game/BP_HUD.CombatUI` (`/Game/ActorComponents/BP_Fleet.Hud` (`self.Fleet`))))))

(fn `GetShipDamage`
  (params (Stat :type "/Game/GlobalEnums/E_TradeGoodProperty Enum" :default "NewEnumerator0"))
  (returns (Value :type Integer))
  (bind (_value _returnvalue) (`BlueprintMapLibrary.Map_Find` (`self.ShipDamage`) Stat))
  (if _returnvalue
    (return _value)
    (else
      (return 0))))

(fn `GetShipStat`
  (params (Stat :type "/Game/GlobalEnums/E_TradeGoodProperty Enum" :default "NewEnumerator0"))
  (returns (Value :type Integer))
  (bind (_value _returnvalue) (`BlueprintMapLibrary.Map_Find` (`self.ShipStats`) Stat))
  (if _returnvalue
    (return _value)
    (else
      (return 0))))

(fn `RollBattleRoll`
  (params (Stat :type "/Game/GlobalEnums/E_BattleTarget Enum" :default "NewEnumerator0"))
  (`BlueprintMapLibrary.Map_Add` (`self.BattleRoll`) Stat (`self.GetBattleStatRoll` Stat)))

(fn `RollDamagePhase`
  (`self.RollBattleRoll` "NewEnumerator2")
  (`self.RollBattleRoll` "NewEnumerator3")
  (switch `/Game/GlobalEnums/E_BattleShipState` (`self.BattleShipState`)
    (:`NewEnumerator0`
      _)
    (:`NewEnumerator1`
      _))
  (`self.RollBattleRoll` "NewEnumerator5"))

(fn `RollManeuverPhase`
  (`self.RollBattleRoll` "NewEnumerator1"))

(fn `SetBattleShipState`
  (params (BattleShipState :type "/Game/GlobalEnums/E_BattleShipState Enum" :default "NewEnumerator0"))
  (bind _output_get (set `self.BattleShipState` BattleShipState))
  (switch `/Game/GlobalEnums/E_BattleShipState` _output_get
    (:`NewEnumerator2`
      (`BlueprintMapLibrary.Map_Add` (`self.BattleRoll`) "NewEnumerator5"))))

(fn `SetupPreviewPhase`
  (`BlueprintMapLibrary.Map_Clear` (`self.BattleRoll`))
  (set `self.BattleShipState` "NewEnumerator1"))