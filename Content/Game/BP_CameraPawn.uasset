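; BP_CameraPawn is a camera pawn that follows the player's fleet and supports zoom, pan and rotation.
; Each Tick it takes the assigned fleet's position as focus, then teleports itself back along the desired view direction by the camera distance, from that focus plus pan offset.
; Input-agnostic functions adjust the clamped zoom distance, yaw and pan offset, with panning relative to camera yaw so it stays horizontal.
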(event `self.ReceiveBeginPlay`)

(event `self.ReceiveTick`
  (params (DeltaSeconds :type "Float (single-precision)"))
  (bind _playerfleet (`self.PlayerFleet`))
  (`|ExecutionSequence`
    (:`then_0`
      (`/Engine/EditorBlueprintResources/StandardMacros.IsValid` _playerfleet
        (:`Is Valid`
          (set `self.ViewFocus` (`/Game/Actors/BP_CampaignFleet.GetCurrentPosition` _playerfleet)))))
    (:`then_1`
      (`self.K2_SetActorTransform` self (`KismetMathLibrary.MakeTransform` (+ (`self.ViewFocus`) (`self.ViewFocusOffset`) (* (`KismetMathLibrary.GetForwardVector` (`self.DesiredRotation`)) -1 (`self.CameraDistance`))) (`self.DesiredRotation`)) false true))))

(fn `IncrementCameraPan`
  (params (Direction :type "Vector2D Structure"))
  (bind (_x _y) (`KismetMathLibrary.BreakVector2D` Direction))
  (bind _newrotation (`/JGGUniversalFunctionsAndMacros/FunctionLibraries/FL_Transformation.RemoveRotationAxis` (`self.DesiredRotation`) true true))
  (set `self.ViewFocusOffset` (+ (* _x (`KismetMathLibrary.GetRightVector` _newrotation)) (* _y (`KismetMathLibrary.GetForwardVector` _newrotation)) (`self.ViewFocusOffset`))))

(fn `IncrementCameraRotation`
  (params (RotationChange :type "Float (double-precision)"))
  (set `self.DesiredRotation` (`KismetMathLibrary.MakeRotator` (.roll (`self.DesiredRotation`)) (.pitch (`self.DesiredRotation`)) (+ (.yaw (`self.DesiredRotation`)) RotationChange))))

(fn `IncrementCameraZoom`
  (params (ZoomChange :type "Float (double-precision)"))
  (set `self.CameraDistance` (`KismetMathLibrary.FClamp` (+ ZoomChange (`self.CameraDistance`)) 100.0 10000.0)))

(fn `SetPlayerFleet`
  (params (Fleet :type "/Game/Actors/BP_CampaignFleet Object Reference"))
  (set `self.PlayerFleet` Fleet))

(fn `UserConstructionScript`)