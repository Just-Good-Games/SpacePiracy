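; Player controller that turns input into camera zoom, pan and rotation and click-to-select location for the game.
; On BeginPlay it caches the camera pawn and the click-location actor from the game mode.
; Axis and button inputs are scaled by multipliers, with pan also scaled by camera distance.
; Left clicks project the mouse ray onto the Z=0 plane, notify the pawn and move the click-location actor there.
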(event `self.ReceiveBeginPlay`
  (bind _asbp_game_mode (cast `/Game/Game/BP_GameMode` (`GameplayStatics.GetGameMode`)))
  (bind _output_get (set `self.GameMode` _asbp_game_mode))
  (set `self.ClickLocation` (`/Game/Game/BP_GameMode.ClickLocation` _output_get))
  (bind _asbp_camera_pawn (cast `/Game/Game/BP_CameraPawn` (`self.K2_GetPawn`)))
  (set `self.CameraPawn` _asbp_camera_pawn))

(event `InputAxis|CameraZoom`
  (params (AxisValue :type "Float (single-precision)"))
  (`self.ApplyCameraZoom` AxisValue))

(event `InputAction|CameraZoomIn`
  (params (Key :type "Key Structure"))
  (:`Pressed`
    (`self.ApplyCameraZoom` 1.0)))

(event `InputAction|CameraZoomOut`
  (params (Key :type "Key Structure"))
  (:`Pressed`
    (`self.ApplyCameraZoom` -1.0)))

(event `InputAxis|PanHorizontal`
  (params (AxisValue :type "Float (single-precision)"))
  (`self.ApplyCameraPan` AxisValue))

(event `InputAction|PanLeft`
  (params (Key :type "Key Structure"))
  (:`Pressed`
    (`self.ApplyCameraPan` -1.0)))

(event `InputAction|PanRight`
  (params (Key :type "Key Structure"))
  (:`Pressed`
    (`self.ApplyCameraPan` 1.0)))

(event `InputAxis|PanVertical`
  (params (AxisValue :type "Float (single-precision)"))
  (`self.ApplyCameraPan` 0.0 AxisValue))

(event `InputAction|PanDown`
  (params (Key :type "Key Structure"))
  (:`Pressed`
    (`self.ApplyCameraPan` 0.0 -1.0)))

(event `InputAction|PanUp`
  (params (Key :type "Key Structure"))
  (:`Pressed`
    (`self.ApplyCameraPan` 0.0 1.0)))

(event `InputAction|LeftClick`
  (params (Key :type "Key Structure"))
  (bind (_worldlocation _worlddirection) (`self.DeprojectMousePositionToWorld`))
  (:`Pressed`
    (`self.ApplyLocationSelected` (+ _worldlocation (* (`KismetMathLibrary.SafeDivide` (.z _worldlocation) (.z _worlddirection)) -1.0 _worlddirection)))))

(event `InputAxis|CameraRotate`
  (params (AxisValue :type "Float (single-precision)"))
  (`self.ApplyCameraRotation` AxisValue))

(event `InputAction|CameraRotateClockwise`
  (params (Key :type "Key Structure"))
  (:`Pressed`
    (`self.ApplyCameraRotation` 1.0)))

(event `InputAction|CameraRotateCounterClockwise`
  (params (Key :type "Key Structure"))
  (:`Pressed`
    (`self.ApplyCameraRotation` -1.0)))

(fn `ApplyCameraPan`
  (params (Horizontal :type "Float (double-precision)") (Vertical :type "Float (double-precision)"))
  (`/Game/Game/BP_CameraPawn.IncrementCameraPan` (`self.CameraPawn`) (* (`KismetMathLibrary.NormalSafe2D` (`KismetMathLibrary.MakeVector2D` Horizontal Vertical)) (* (`self.PanningMultiplier`) (`/Game/Game/BP_CameraPawn.CameraDistance` (`self.CameraPawn`))))))

(fn `ApplyCameraRotation`
  (params (Axis :type "Float (double-precision)"))
  (`/Game/Game/BP_CameraPawn.IncrementCameraRotation` (`self.CameraPawn`) (* Axis (`self.RotationMultiplier`))))

(fn `ApplyCameraZoom`
  (params (Axis :type "Float (double-precision)"))
  (`/Game/Game/BP_CameraPawn.IncrementCameraZoom` (`self.CameraPawn`) (* Axis (`self.ZoomMultiplier`))))

(fn `ApplyLocationSelected`
  (params (Location :type "Vector Structure"))
  (`/Game/Game/BP_CameraPawn.LocationSelected` (`self.CameraPawn`) Location)
  (`self.K2_SetActorLocation` (`self.ClickLocation`) Location false true))

(fn `UserConstructionScript`)