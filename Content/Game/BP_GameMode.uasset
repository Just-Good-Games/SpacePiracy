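; Game mode for a fleet campaign game that owns player settings, pausing and frame-budgeted processing of battles and fleet creation.
; On BeginPlay it loads or creates the settings save, triggers a settings update, spawns the click location actor and hands the campaign manager to the tutorial.
; Tick, kept running while paused, drains queued battles and fleets through capped per-frame turn and ship-creation calls, removing each when it reports done.
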(event `self.ReceiveBeginPlay`
  (`|ExecutionSequence`
    (:`then_0`
      (bind _returnvalue (`GameplayStatics.LoadGameFromSlot` (`self.SettingsSaveFile`)))
      (bind _asbp_settings_save (cast `/Game/Objects/BP_SettingsSave` _returnvalue)
        (:`then`
          (bind _output_get (set `self.Settings` _asbp_settings_save))
          (`/Engine/EditorBlueprintResources/StandardMacros.IsValid` _output_get
            (:`Is Not Valid`
              _)))
        (:`CastFailed`
          _))
      (bind _returnvalue_2 (`|GenericCreateObject` "/Game/Objects/BP_SettingsSave.BP_SettingsSave_C"))
      (set `self.Settings` _returnvalue_2))
    (:`then_1`
      (`self.SettingUpdate`))
    (:`then_2`
      (bind _returnvalue_3 (`|SpawnActorFromClass` "/Game/Actors/BP_ClickLocation.BP_ClickLocation_C" (`KismetMathLibrary.MakeTransform` (0.0 0.0 0.0)) "Undefined" "MultiplyWithRoot" null null))
      (set `self.ClickLocation` _returnvalue_3)
      (set `/Game/ActorComponents/BP_SpaceTutorial.CampaignManager` (`self.CampaignManager`) (`self.CampaignTutorial`))
      (`self.SetTickableWhenPaused` true))))

(event `self.ReceiveTick`
  (params (DeltaSeconds :type "Float (single-precision)"))
  (bind _queuedbattles (`self.QueuedBattles`))
  (bind _queuedfleets (`self.QueuedFleets`))
  (`|ExecutionSequence`
    (:`then_0`
      (for _ (range 1 (+ (`self.MaxBattlesPerFrame`) 1))
        (if (<= (`KismetArrayLibrary.Array_Length` _queuedbattles) 0)
          (break)
          (else
            (bind _bbattleover (`/Game/Objects/BP_Battle.ResolveTurn` (`|GetArrayItem` _queuedbattles)))
            (if _bbattleover
              (`KismetArrayLibrary.Array_Remove` (`self.QueuedBattles`)))))))
    (:`then_1`
      (for _ (range 1 (+ (`self.MaxShipsPerFrame`) 1))
        (if (<= (`KismetArrayLibrary.Array_Length` _queuedfleets) 0)
          (break)
          (else
            (bind _fleetfinished (`/Game/ActorComponents/BP_Fleet.CreateQueuedShip` (`|GetArrayItem` _queuedfleets)))
            (if _fleetfinished
              (`KismetArrayLibrary.Array_Remove` (`self.QueuedFleets`)))))))))

(fn `QueueBattle`
  (params (Battle :type "/Game/Objects/BP_Battle Object Reference"))
  (`KismetArrayLibrary.Array_Add` (`self.QueuedBattles`) Battle))

(fn `QueueFleet`
  (params (Fleet :type "/Game/ActorComponents/BP_Fleet Object Reference"))
  (`KismetArrayLibrary.Array_Add` (`self.QueuedFleets`) Fleet))

(fn `SaveSettings`
  (`GameplayStatics.SaveGameToSlot` (`self.Settings`) (`self.SettingsSaveFile`))
  (`self.SettingUpdate`))

(fn `SetPauseState`
  (params (bPaused :type Boolean))
  (`GameplayStatics.SetGamePaused` bPaused))

(fn `UserConstructionScript`)