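; Solar system actor for the campaign map, building one system from its SolarSystemData and drawing its slipstream links.
; BeginPlay adds stars and planets from DataTables, spawns campaign fleets when GeneratedShips is set, and flags whether the player's fleet is present.
; After a zero-second delay, slipstream endpoints are computed edge to edge with systems found in CampaignManager.
; Tick debug-draws those links, adding boundary and entry circles in the player's system.
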(event `self.ReceiveBeginPlay`
  (`self.SetupStars`)
  (`self.SetupPlanets`)
  (`self.SetupShips`)
  (`KismetSystemLibrary.Delay` 0.0)
  (`self.SetupSlipStream`))

(event `self.ReceiveTick`
  (params (DeltaSeconds :type "Float (single-precision)"))
  (`self.DrawSlipStream`)
  (if (`self.ContainsPlayer`)
    (`self.DrawSystemEdge`)))

(fn `ContainsPlayer`
  (returns (bContainsPlayer :type Boolean))
  (return (`self.bContainsPlayer`)))

(fn `DrawSlipStream`
  (locals (StartLocation :type "Vector Structure") (MiddleLocation :type "Vector Structure") (EndLocation :type "Vector Structure"))
  (for (_array_element _array_index) (`self.SlipStreamStarts`)
    (set `local.StartLocation` _array_element)
    (set `local.EndLocation` (`|GetArrayItem` (`self.SlipStreamEnds`) _array_index))
    (set `local.MiddleLocation` (/ (+ (`local.StartLocation`) (`local.EndLocation`)) 2.0))
    (`KismetSystemLibrary.DrawDebugArrow` (`local.StartLocation`) (`local.MiddleLocation`) 10000000.0 (struct :`R` 1.0 :`G` 1.0 :`B` 1.0 :`A` 1.0))
    (`KismetSystemLibrary.DrawDebugArrow` (`local.MiddleLocation`) (`local.EndLocation`) 10000000.0 (struct :`R` 1.0 :`G` 1.0 :`B` 1.0 :`A` 1.0))
    (if (`self.bContainsPlayer`)
      (`KismetSystemLibrary.DrawDebugCircle` (`local.StartLocation`) (`self.SlipStreamRadius`) 8 (struct :`R` 1.0 :`G` 1.0 :`B` 1.0 :`A` 1.0) 0.0 0.0 (0.0 1.0 0.0) (1.0 0.0 0.0)))))

(fn `DrawSystemEdge`
  (`KismetSystemLibrary.DrawDebugCircle` (`self.K2_GetActorLocation`) (`.Radius_58_FF405E09454FF9C40FC9808B1FC38F34` (break `/Game/Structs/S_SolarSystemData` (`self.SolarSystemData`))) 64 (struct :`R` 1.0 :`G` 1.0 :`B` 1.0 :`A` 1.0) 0.0 0.0 (0.0 1.0 0.0) (1.0 0.0 0.0)))

(fn `SetupPlanets`
  (bind (_name _slipstreams _stars _planets _fleetinstances _position _radius) (break `/Game/Structs/S_SolarSystemData` (`self.SolarSystemData`)))
  (for _array_element _planets
    (bind _returnvalue (`|GetDataTableRow` "/Game/DataTables/DT_Planets.DT_Planets" _array_element)
      (:`then`
        (bind (_name_2 _faction _production _wealth _weight _defensetemplate _position_2 _radius_2) (break `/Game/Structs/S_PlanetData` _returnvalue))
        (bind _returnvalue_2 (`|AddComponentByClass` "/Game/SceneComponents/BP_Planet.BP_Planet_C" false (`/JGGUniversalFunctionsAndMacros/FunctionLibraries/FL_Transformation.Relative2DToWorldTransform3D` (`self.K2_GetActorLocation`) _position_2 _radius (/ _radius_2 50.0)) _returnvalue))
        (`KismetArrayLibrary.Array_Add` (`self.Planets`) _returnvalue_2)))))

(fn `SetupShips`
  (bind (_name _slipstreams _stars _planets _fleetinstances _position _radius) (break `/Game/Structs/S_SolarSystemData` (`self.SolarSystemData`)))
  (if (`self.bGeneratedShips`)
    (for _array_element _fleetinstances
      (bind (_fleettemplate _faction _position_2) (break `/Game/Structs/S_FleetInstanceData` _array_element))
      (bind _returnvalue (== _fleettemplate (`self.PlayerName`)))
      (bind _returnvalue_2 (`|SpawnActorFromClass` "/Game/Actors/BP_CampaignFleet.BP_CampaignFleet_C" (`/JGGUniversalFunctionsAndMacros/FunctionLibraries/FL_Transformation.Relative2DToWorldTransform3D` (`self.K2_GetActorLocation`) _position_2 _radius) "Undefined" "MultiplyWithRoot" null _fleettemplate _returnvalue _faction null))
      (`KismetArrayLibrary.Array_Add` (`self.Fleets`) _returnvalue_2)
      (if _returnvalue
        (set `self.bContainsPlayer` true)))))

(fn `SetupSlipStream`
  (locals (OtherSystem :type "/Game/Actors/BP_SolarSystem Object Reference"))
  (bind _returnvalue (`KismetMathLibrary.GetDirectionUnitVector` (`self.K2_GetActorLocation`) (`self.K2_GetActorLocation` (`local.OtherSystem`))))
  (for _array_element (`.SlipStreams_50_0EAB655A4AD153C23A6A32929751D735` (break `/Game/Structs/S_SolarSystemData` (`self.SolarSystemData`)))
    (bind (_value _returnvalue_2) (`BlueprintMapLibrary.Map_Find` (`/Game/ActorComponents/BP_CampaignManager.SolarSystems` (`self.CampaignManager`)) _array_element))
    (if _returnvalue_2
      (set `local.OtherSystem` _value)
      (`KismetArrayLibrary.Array_Add` (`self.SlipStreamStarts`) (+ (`self.K2_GetActorLocation`) (* _returnvalue (`.Radius_58_FF405E09454FF9C40FC9808B1FC38F34` (break `/Game/Structs/S_SolarSystemData` (`self.SolarSystemData`))))))
      (`KismetArrayLibrary.Array_Add` (`self.SlipStreamEnds`) (- (`self.K2_GetActorLocation` (`local.OtherSystem`)) (* _returnvalue (`.Radius_58_FF405E09454FF9C40FC9808B1FC38F34` (break `/Game/Structs/S_SolarSystemData` (`/Game/Actors/BP_SolarSystem.SolarSystemData` (`local.OtherSystem`))))))))))

(fn `SetupStars`
  (bind (_name _slipstreams _stars _planets _fleetinstances _position _radius) (break `/Game/Structs/S_SolarSystemData` (`self.SolarSystemData`)))
  (for _array_element _stars
    (bind _returnvalue (`|GetDataTableRow` "/Game/DataTables/DT_Stars.DT_Stars" _array_element)
      (:`then`
        (bind (_name_2 _color _position_2 _radius_2) (break `/Game/Structs/S_StarData` _returnvalue))
        (bind _returnvalue_2 (`|AddComponentByClass` "/Game/SceneComponents/BP_Star.BP_Star_C" false (`/JGGUniversalFunctionsAndMacros/FunctionLibraries/FL_Transformation.Relative2DToWorldTransform3D` (0.0 0.0 0.0) _position_2 _radius (/ _radius_2 50.0)) _returnvalue))
        (`KismetArrayLibrary.Array_Add` (`self.Stars`) _returnvalue_2)))))

(fn `UserConstructionScript`)