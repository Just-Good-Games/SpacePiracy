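; BP_UnitTester is an actor that runs in-game sanity checks on trade good and map helper logic.
; RunUnitTests chains UnitTest calls that compare GetTradeGoodProperty results (shield price, forward battery, armor) and IncrementIntegerMap return and stored values against expected numbers.
; A sequence brackets the checks with start and end messages and clears the ShipStats scratch map afterward.
; Its event graph is empty, so nothing here triggers the tests.
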(fn `RunUnitTests`
  (bind (_value _returnvalue) (`BlueprintMapLibrary.Map_Find` (`self.ShipStats`) "NewEnumerator2"))
  (bind (_value_2 _returnvalue_2) (`BlueprintMapLibrary.Map_Find` (`self.ShipStats`) "NewEnumerator2"))
  (`|ExecutionSequence`
    (:`then_0`
      (`/JGGErrorAndTesting/FunctionLibraries/FL_Error.PrintMessage` null "NewEnumerator0" "Start Of Unit Tests"))
    (:`then_1`
      (`/JGGErrorAndTesting/Macros/BM_UnitTests.UnitTest` (`/Game/FunctionLibraries/FL_TradeGoods.GetTradeGoodProperty` "NewEnumerator6" "NewEnumerator2" "NewEnumerator3" 3) 16 "" "NewEnumerator1" "Shield Price Calc Not Working"
        (:`ExecOut`
          (`/JGGErrorAndTesting/Macros/BM_UnitTests.UnitTest` (`/Game/FunctionLibraries/FL_TradeGoods.GetTradeGoodProperty` "NewEnumerator4" "NewEnumerator6" "NewEnumerator1" 5) 30 "" "NewEnumerator1" "Forward Battery Calc Not Working"
            (:`ExecOut`
              (`/JGGErrorAndTesting/Macros/BM_UnitTests.UnitTest` (`/Game/FunctionLibraries/FL_TradeGoods.GetTradeGoodProperty` "NewEnumerator8" "NewEnumerator6" "NewEnumerator1" 5) 0 "" "NewEnumerator1" "Invalid Armor Calc Not Working"
                (:`ExecOut`
                  (bind _newvalue (`/JGGUniversalFunctionsAndMacros/Macros/BM_Maps.IncrementIntegerMap` (`self.ShipStats`) "NewEnumerator2" 1)
                    (:`OutExec`
                      (`/JGGErrorAndTesting/Macros/BM_UnitTests.UnitTest` _newvalue 1 "" "NewEnumerator1" "Invalid Increment Map - Return"
                        (:`ExecOut`
                          (`/JGGErrorAndTesting/Macros/BM_UnitTests.UnitTest` (select `bool` _returnvalue_2 :`true` _value_2) 1 "" "NewEnumerator1" "Invalid Increment Map - Stored"
                            (:`ExecOut`
                              (bind _newvalue_2 (`/JGGUniversalFunctionsAndMacros/Macros/BM_Maps.IncrementIntegerMap` (`self.ShipStats`) "NewEnumerator2" 1)
                                (:`OutExec`
                                  (`/JGGErrorAndTesting/Macros/BM_UnitTests.UnitTest` _newvalue_2 2 "" "NewEnumerator1" "Invalid Increment Map - Return"
                                    (:`ExecOut`
                                      (`/JGGErrorAndTesting/Macros/BM_UnitTests.UnitTest` (select `bool` _returnvalue :`true` _value) 2 "" "NewEnumerator1" "Invalid Increment Map - Stored"))))))))))))))))))
    (:`then_2`
      (`BlueprintMapLibrary.Map_Clear` (`self.ShipStats`)))
    (:`then_3`
      (`/JGGErrorAndTesting/FunctionLibraries/FL_Error.PrintMessage` null "NewEnumerator0" "End Of Unit Tests"))))

(fn `UserConstructionScript`)