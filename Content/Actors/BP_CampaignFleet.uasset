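; Campaign-map fleet actor that carries a FleetComponent and flies between destinations in solar systems and slipstreams, for the player or AI.
; A navigation object, chosen by player flag, campaign type and fleet type, sets the destination each tick.
; Movement uses Newton's-method intercept thrust in systems and fixed-direction velocity in slipstreams, scaled by fleet stats.
; Reaching another fleet starts a cooldown-gated BP_Battle; reaching slipstreams or tutorial markers triggers their handlers.
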(event `self.ReceiveBeginPlay`
  (set `self.TimeSinceLastFight` (`self.MinimumTimeBetweenBattles`))
  (add `/Game/ActorComponents/BP_Fleet.OnFleetDestroyed` (`self.FleetComponent`) (`|CreateDelegate` :!event `OnFleetDestroyed`))
  (bind _asbp_player_controller (cast `/Game/Game/BP_PlayerController` (`GameplayStatics.GetPlayerController` 0) :!label _label)
    (:`then`
      (bind _output_get (set `self.PlayerController` _asbp_player_controller))
      (bind _output_get_2 (set `self.CameraPawn` (`/Game/Game/BP_PlayerController.CameraPawn` _output_get)))
      (`/Engine/EditorBlueprintResources/StandardMacros.IsValid` _output_get_2
        (:`Is Valid`
          (if (`self.bHumanPlayer`)
            (`/Game/Game/BP_CameraPawn.SetPlayerFleet` (`self.CameraPawn`) self)))
        (:`Is Not Valid`
          (`KismetSystemLibrary.Delay` 0.1 :!label _label_2)
          (goto _label))))
    (:`CastFailed`
      (goto _label_2))))

(event `self.ReceiveTick`
  (params (DeltaSeconds :type "Float (single-precision)"))
  (`/Engine/EditorBlueprintResources/StandardMacros.IsValid` self
    (:`Is Valid`
      (`|ExecutionSequence`
        (:`then_0`
          (set `self.TimeSinceLastFight` (+ DeltaSeconds (`self.TimeSinceLastFight`))))
        (:`then_1`
          (`/Game/Objects/BP_AINav_Base.SetDestination` (`self.AINavigation`))
          (`self.CheckForDestinationReached`))
        (:`then_2`
          (`/Engine/EditorBlueprintResources/StandardMacros.IsValid` self
            (:`Is Valid`
              (`/Engine/EditorBlueprintResources/StandardMacros.IsValid` (`self.SlipStream`)
                (:`Is Valid`
                  (`self.DetermineMovementSlipStream`))
                (:`Is Not Valid`
                  (`self.MovementSolarSystem`))))))))))

(event `/Game/Interfaces/BI_NavigationSelectable.DestroyNavigatable`
  (bind _camerapawn (`self.CameraPawn`))
  (bind _playercontroller (`self.PlayerController`))
  (bind _solarsystem (`self.SolarSystem`))
  (`|ExecutionSequence`
    (:`then_0`
      (if (`self.bHumanPlayer`)
        (`/Engine/EditorBlueprintResources/StandardMacros.IsValid` _camerapawn
          (:`Is Valid`
            (set `/Game/Game/BP_CameraPawn.PlayerFleet` null _camerapawn)
            (`/Engine/EditorBlueprintResources/StandardMacros.IsValid` _playercontroller
              (:`Is Valid`
                (`self.SetActorHiddenInGame` (`/Game/Game/BP_PlayerController.ClickLocation` _playercontroller) true)))))))
    (:`then_1`
      (`KismetArrayLibrary.Array_RemoveItem` (`/Game/Actors/BP_SolarSystem.Clickables` _solarsystem) self)
      (`KismetArrayLibrary.Array_RemoveItem` (`/Game/Actors/BP_SolarSystem.Fleets` _solarsystem) self)
      (`self.K2_DestroyActor`))))

(fn `ApplyMovementSlipStream`
  (params (bMove :type Boolean))
  (locals (Velocity :type "Vector Structure"))
  (`|ExecutionSequence`
    (:`then_0`
      (if bMove
        (set `local.Velocity` (* (`self.GetSlipStreamSpeed`) (`/Game/SceneComponents/BP_SlipStream.UnitDirection` (`self.SlipStream`))))
        (`self.SetArrowVisible` true)
        (else
          (set `local.Velocity` (0.0 0.0 0.0))
          (`self.SetArrowVisible` false))))
    (:`then_1`
      (`PrimitiveComponent.SetPhysicsLinearVelocity` (`self.MovingComponent`) (`local.Velocity`) false "None"))))

(fn `ChangeSolarSystem`
  (params (NewSolarSystem :type "/Game/Actors/BP_SolarSystem Object Reference"))
  (bind _playercontroller (`self.PlayerController`))
  (bind _clicklocation (`/Game/Game/BP_PlayerController.ClickLocation` _playercontroller))
  (`|ExecutionSequence`
    (:`then_0`
      (`/Game/Actors/BP_SolarSystem.RemoveFleet` (`self.SolarSystem`) self)
      (`/Game/Actors/BP_SolarSystem.AddFleet` (`local.NewSolarSystem`) self))
    (:`then_1`
      (set `self.SolarSystem` NewSolarSystem))
    (:`then_2`
      (if (`self.bHumanPlayer`)
        (`/Engine/EditorBlueprintResources/StandardMacros.IsValid` _playercontroller
          (:`Is Valid`
            (`self.K2_SetActorLocation` _clicklocation (* (+ (`self.GetCurrentPosition`) (`self.K2_GetActorLocation` (`self.SolarSystem`))) 0.5) false true)
            (set `self.DestinationObject` _clicklocation)))))))

(fn `CheckForDestinationReached`
  (bind _destinationobject (`self.DestinationObject`))
  (`/Engine/EditorBlueprintResources/StandardMacros.IsValid` (`KismetSystemLibrary.Conv_InterfaceToObject` (`self.DestinationObject`))
    (:`Is Valid`
      (bind _radius (`/Game/Interfaces/BI_NavigationSelectable.GetRadius` self))
      (bind _location (`/Game/Interfaces/BI_NavigationSelectable.GetLocation` self))
      (bind _radius_2 (`/Game/Interfaces/BI_NavigationSelectable.GetRadius` _destinationobject))
      (bind _location_2 (`/Game/Interfaces/BI_NavigationSelectable.GetLocation` _destinationobject))
      (bind _bcollision (`/JGGUniversalFunctionsAndMacros/FunctionLibraries/FL_Transformation.SimpleCircleCollisionCheck2D` _location_2 _radius_2 _location _radius))
      (if _bcollision
        (`self.OnDestinationReached`)))))

(fn `DetermineMovementSlipStream`
  (bind _destinationobject (`self.DestinationObject`))
  (`/Engine/EditorBlueprintResources/StandardMacros.IsValid` (`KismetSystemLibrary.Conv_InterfaceToObject` _destinationobject)
    (:`Is Valid`
      (cast `/Game/SceneComponents/BP_SlipStream` _destinationobject
        (:`then`
          (`self.ApplyMovementSlipStream` true :!label _label))
        (:`CastFailed`
          (bind _location (`/Game/Interfaces/BI_NavigationSelectable.GetLocation` _destinationobject))
          (`self.ApplyMovementSlipStream` (> (`KismetMathLibrary.Dot_VectorVector` (- _location (`self.GetCurrentPosition`)) (`/Game/SceneComponents/BP_SlipStream.UnitDirection` (`self.SlipStream`))) 0.0)))))
    (:`Is Not Valid`
      (goto _label))))

(fn `GetAbleToBattle`
  (returns (bAbleToBattle :type Boolean))
  (return (>= (`self.TimeSinceLastFight`) (`self.MinimumTimeBetweenBattles`))))

(fn `GetAccelerationScalar`
  (returns (Value :type "Float (single-precision)"))
  (bind _fleetcomponent (`self.FleetComponent`))
  (return (* (`self.SpeedImpulseScale`) (`KismetMathLibrary.SafeDivide` (`KismetMathLibrary.Conv_IntToDouble` (`/Game/ActorComponents/BP_Fleet.GetFleetStats` _fleetcomponent "NewEnumerator9")) (`KismetMathLibrary.Conv_IntToDouble` (`/Game/ActorComponents/BP_Fleet.GetFleetStats` _fleetcomponent "NewEnumerator1"))))))

(fn `GetAccelerationVector`
  (returns (Force :type "Vector Structure"))
  (return (* (`self.GetAccelerationScalar`) (`self.GetDirection`))))

(fn `GetAttachableComponent`
  (returns (Component :type "SceneComponent Object Reference"))
  (return (`self.MovingComponent`)))

(fn `GetCurrentPosition`
  (returns (Value :type "Vector Structure"))
  (return (`SceneComponent.K2_GetComponentLocation` (`self.MovingComponent`))))

(fn `GetCurrentVelocity`
  (returns (Value :type "Vector Structure"))
  (return (`SceneComponent.GetComponentVelocity` (`self.MovingComponent`))))

(fn `GetDestination`
  (returns (Destination :type "Vector Structure"))
  (bind _destinationobject (`self.DestinationObject`))
  (`/Engine/EditorBlueprintResources/StandardMacros.IsValid` (`KismetSystemLibrary.Conv_InterfaceToObject` _destinationobject)
    (:`Is Valid`
      (bind _location (`/Game/Interfaces/BI_NavigationSelectable.GetLocation` _destinationobject))
      (return _location))
    (:`Is Not Valid`
      (return (`self.GetCurrentPosition`)))))

(fn `GetDirection`
  (returns (Direction :type "Vector Structure"))
  (locals (Directions :type "Array of Vector Structure") (DirectionToTarget :type "Vector Structure") (VelocityPortion :type "Float (double-precision)" :default 0.0) (VelocityPortionAcceleration :type "Vector Structure") (FinalDirection :type "Vector Structure") (Displacement :type "Vector Structure") (ChangeInVelocity :type "Vector Structure") (FinalVelocity :type "Vector Structure") (CounterToVelocity :type "Vector Structure" :default (0.0 0.0 0.0)) (VelocityProportion :type "Float (double-precision)" :default 0.5))
  (bind _direction (`/Game/FunctionLibraries/FL_RocketCalculations.RocketInterceptDirection_NewtonsMeth` (`self.GetRelativePositionOfTarget`) (`self.GetRelativeVelocityOfTarget`) (`self.GetAccelerationScalar`) self))
  (return _direction))

(fn `GetLocation`
  (returns (Location :type "Vector Structure"))
  (return (`self.GetCurrentPosition`)))

(fn `GetRadius`
  (returns (Radius :type "Float (double-precision)"))
  (return (`SphereComponent.SphereRadius` (`self.MovingComponent`))))

(fn `GetRelativePositionOfTarget`
  (returns (Position :type "Vector Structure"))
  (bind _destinationobject (`self.DestinationObject`))
  (`/Engine/EditorBlueprintResources/StandardMacros.IsValid` (`KismetSystemLibrary.Conv_InterfaceToObject` _destinationobject)
    (:`Is Valid`
      (bind _location (`/Game/Interfaces/BI_NavigationSelectable.GetLocation` _destinationobject))
      (return (- _location (`self.GetCurrentPosition`))))
    (:`Is Not Valid`
      (return (0.0 0.0 0.0)))))

(fn `GetRelativeVelocityOfTarget`
  (returns (Velocity :type "Vector Structure"))
  (bind _destinationobject (`self.DestinationObject`))
  (`/Engine/EditorBlueprintResources/StandardMacros.IsValid` (`KismetSystemLibrary.Conv_InterfaceToObject` _destinationobject)
    (:`Is Valid`
      (bind _velocity (`/Game/Interfaces/BI_NavigationSelectable.GetVelocityIfAny` _destinationobject))
      (return (- _velocity (`self.GetCurrentVelocity`))))
    (:`Is Not Valid`
      (return (0.0 0.0 0.0)))))

(fn `GetSlipStreamSpeed`
  (returns (Speed :type "Float (double-precision)"))
  (bind _fleetcomponent (`self.FleetComponent`))
  (return (* (`self.SpeedSlipStreamScale`) (`KismetMathLibrary.SafeDivide` (`KismetMathLibrary.Conv_IntToDouble` (`/Game/ActorComponents/BP_Fleet.GetFleetStats` _fleetcomponent "NewEnumerator12")) (`KismetMathLibrary.Conv_IntToDouble` (`/Game/ActorComponents/BP_Fleet.GetFleetStats` _fleetcomponent "NewEnumerator1"))))))

(fn `GetVelocityIfAny`
  (returns (Velocity :type "Vector Structure"))
  (return (`self.GetCurrentVelocity`)))

(fn `MovementSolarSystem`
  (bind _solarsystem (`self.SolarSystem`))
  (`PrimitiveComponent.AddForce` (`self.MovingComponent`) (`self.GetAccelerationVector`) "None" true)
  (`/Engine/EditorBlueprintResources/StandardMacros.IsValid` _solarsystem
    (:`Is Valid`
      (if (`/Game/Actors/BP_SolarSystem.ContainsPlayer` _solarsystem)
        (`SceneComponent.K2_SetWorldRotation` (`self.MovingComponent`) (`KismetMathLibrary.FindLookAtRotation` (`KismetMathLibrary.Vector_Zero`) (`self.GetDirection`)) false false)
        (`SceneComponent.K2_SetWorldRotation` (`self.VelocityArrow`) (`KismetMathLibrary.FindLookAtRotation` (`KismetMathLibrary.Vector_Zero`) (`self.GetCurrentVelocity`)) false false)
        (`self.SetArrowVisible` true)))))

(fn `OnDestinationReached`
  (bind _solarsystem (`self.SolarSystem`))
  (bind _slipstream (`self.SlipStream`))
  (bind _solarsystem_2 (`self.SolarSystem`))
  (bind _destinationobject (`self.DestinationObject`))
  (bind _campaignmanager (`/Game/Actors/BP_SolarSystem.CampaignManager` _solarsystem))
  (bind _hud (`/Game/ActorComponents/BP_CampaignManager.HUD` _campaignmanager))
  (bind _gamemode (`/Game/Game/BP_HUD.Gamemode` _hud))
  (bind _asbp_campaign_fleet (cast `/Game/Actors/BP_CampaignFleet` _destinationobject)
    (:`then`
      (if (or (`self.GetAbleToBattle`) (`self.GetAbleToBattle` _asbp_campaign_fleet))
        (set `self.TimeSinceLastFight` 0.0)
        (set `/Game/Actors/BP_CampaignFleet.TimeSinceLastFight` 0.0 _asbp_campaign_fleet)
        (`/Engine/EditorBlueprintResources/StandardMacros.IsValid` _solarsystem
          (:`Is Valid`
            (`/Engine/EditorBlueprintResources/StandardMacros.IsValid` _campaignmanager
              (:`Is Valid`
                (`/Engine/EditorBlueprintResources/StandardMacros.IsValid` _hud
                  (:`Is Valid`
                    (`/Engine/EditorBlueprintResources/StandardMacros.IsValid` _gamemode
                      (:`Is Valid`
                        (`PrimitiveComponent.SetPhysicsLinearVelocity` (`self.MovingComponent`) (0.0 0.0 0.0) false "None")
                        (bind _returnvalue (`|GenericCreateObject` "/Game/Objects/BP_Battle.BP_Battle_C" (`|MakeArray` (`self.FleetComponent`)) (`|MakeArray` (`/Game/Actors/BP_CampaignFleet.FleetComponent` _asbp_campaign_fleet)) true _hud _gamemode))
                        (`/Game/Objects/BP_Battle.StartBattle` _returnvalue))
                      (:`Is Not Valid`
                        (`/JGGErrorAndTesting/FunctionLibraries/FL_Error.PrintMessage` self "NewEnumerator1" "Campaign Battle Failed - No Gamemode"))))
                  (:`Is Not Valid`
                    (`/JGGErrorAndTesting/FunctionLibraries/FL_Error.PrintMessage` self "NewEnumerator1" "Campaign Battle Failed - No HUD"))))
              (:`Is Not Valid`
                (`/JGGErrorAndTesting/FunctionLibraries/FL_Error.PrintMessage` self "NewEnumerator1" "Campaign Battle Failed - No Campaign Manager"))))
          (:`Is Not Valid`
            (`/JGGErrorAndTesting/FunctionLibraries/FL_Error.PrintMessage` self "NewEnumerator1" "Campaign Battle Failed - No Solar System")))))
    (:`CastFailed`
      (bind _asbp_tutorial_destination (cast `/Game/SceneComponents/BP_TutorialDestination` _destinationobject)
        (:`then`
          (`/Engine/EditorBlueprintResources/StandardMacros.IsValid` _solarsystem_2
            (:`Is Valid`
              (`KismetArrayLibrary.Array_RemoveItem` (`/Game/Actors/BP_SolarSystem.Clickables` _solarsystem_2) (`self.DestinationObject`))
              (`/Game/SceneComponents/BP_TutorialDestination.OnFleetReached` _asbp_tutorial_destination))))
        (:`CastFailed`
          (bind _asbp_slip_stream (cast `/Game/SceneComponents/BP_SlipStream` _destinationobject)
            (:`then`
              (`/Engine/EditorBlueprintResources/StandardMacros.IsValid` (`self.SlipStream`)
                (:`Is Not Valid`
                  (bind _output_get (set `self.SlipStream` _asbp_slip_stream))
                  (`/Game/SceneComponents/BP_SlipStream.OnFleetReached` _output_get self)
                  (`self.UpdateFleetLocation` (`/Game/SceneComponents/BP_SlipStream.StartLocation` _slipstream))
                  (`SceneComponent.K2_SetWorldRotation` (`self.MovingComponent`) (`KismetMathLibrary.FindLookAtRotation` (`KismetMathLibrary.Vector_Zero`) (`/Game/SceneComponents/BP_SlipStream.UnitDirection` _slipstream)) false false)
                  (`SceneComponent.K2_SetRelativeRotation` :`self` (`self.VelocityArrow`)))))
            (:`CastFailed`
              (bind _asbp_tutorial_aidestination (cast `/Game/SceneComponents/BP_TutorialAIDestination` _destinationobject))
              (`/Game/SceneComponents/BP_TutorialAIDestination.FleetReached` _asbp_tutorial_aidestination)
              (`self.OnFleetDestroyed` self))))))))

(fn `OnFleetDestroyed`
  (if (`self.bHumanPlayer`)
    (`/Game/ActorComponents/BP_CampaignManager.DestroyCampaignMap` (`/Game/Actors/BP_SolarSystem.CampaignManager` (`self.SolarSystem`)))
    (else
      (`/Game/Interfaces/BI_NavigationSelectable.DestroyNavigatable`))))

(fn `SetArrowVisible`
  (params (bNewVisibility :type Boolean))
  (`SceneComponent.SetVisibility` (`self.VelocityArrow`) bNewVisibility false)
  (`SceneComponent.SetVisibility` (`self.AccelerationArrow`) bNewVisibility false))

(fn `SetupMaterials`
  (bind _velocityarrow (`self.VelocityArrow`))
  (bind _accelerationarrow (`self.AccelerationArrow`))
  (bind _gamemode (`/Game/Game/BP_HUD.Gamemode` (`/Game/ActorComponents/BP_CampaignManager.HUD` (`/Game/Actors/BP_SolarSystem.CampaignManager` (`self.SolarSystem`)))))
  (bind _returnvalue (`PrimitiveComponent.CreateDynamicMaterialInstance` _velocityarrow 0 (`PrimitiveComponent.GetMaterial` _velocityarrow 0) "None"))
  (`MaterialInstanceDynamic.SetVectorParameterValue` _returnvalue "Color" (`KismetMathLibrary.Conv_ColorToLinearColor` (`/Game/FunctionLibraries/FL_Factions.GetFactionColor` "NewEnumerator2" _gamemode)))
  (bind _returnvalue_2 (`PrimitiveComponent.CreateDynamicMaterialInstance` _accelerationarrow 0 (`PrimitiveComponent.GetMaterial` _accelerationarrow 0) "None"))
  (`MaterialInstanceDynamic.SetVectorParameterValue` _returnvalue_2 "Color" (`KismetMathLibrary.Conv_ColorToLinearColor` (`/Game/FunctionLibraries/FL_Factions.GetFactionColor` "NewEnumerator1" _gamemode))))

(fn `UpdateFleetLocation`
  (params (NewLocation :type "Vector Structure"))
  (`PrimitiveComponent.SetPhysicsLinearVelocity` (`self.MovingComponent`) (0.0 0.0 0.0) false "None")
  (`SceneComponent.K2_SetWorldLocation` (`self.MovingComponent`) NewLocation false true))

(fn `UserConstructionScript`
  (locals (AINavigationClass :type "/Game/Objects/BP_AINav_Base Class Reference"))
  (bind _fleetcomponent (`self.FleetComponent`))
  (set `/Game/ActorComponents/BP_Fleet.FleetTemplate` (`self.FleetTemplate`) _fleetcomponent)
  (set `/Game/ActorComponents/BP_Fleet.Faction` (`self.Faction`) _fleetcomponent)
  (set `/Game/ActorComponents/BP_Fleet.bIsPlayer` (`self.bHumanPlayer`) _fleetcomponent)
  (set `/Game/ActorComponents/BP_Fleet.Hud` (`/Game/ActorComponents/BP_CampaignManager.HUD` (`/Game/Actors/BP_SolarSystem.CampaignManager` (`self.SolarSystem`))) _fleetcomponent)
  (`/Game/ActorComponents/BP_Fleet.CreateShipsFromFleetTemplate` _fleetcomponent)
  (`self.SetupMaterials`)
  (`|ExecutionSequence`
    (:`then_0`
      (if (`self.bHumanPlayer`)
        (set `local.AINavigationClass` "/Game/Objects/BP_AINav_Player.BP_AINav_Player_C")
        (else
          (switch `/Game/GlobalEnums/E_Campaigns` (`/Game/ActorComponents/BP_CampaignManager.CampaignType` (`/Game/Actors/BP_SolarSystem.CampaignManager` (`self.SolarSystem`)))
            (:`NewEnumerator1`
              (switch `/Game/GlobalEnums/E_FleetType` (`/Game/ActorComponents/BP_Fleet.FleetType` (`self.FleetComponent`))
                (:`NewEnumerator0`
                  (set `local.AINavigationClass` "/Game/Objects/BP_AINav_TutorialPirate.BP_AINav_TutorialPirate_C"))
                (:`NewEnumerator1`
                  (set `local.AINavigationClass` "/Game/Objects/BP_AINav_TutorialMerchant.BP_AINav_TutorialMerchant_C"))))
            (:`NewEnumerator2`
              (set `local.AINavigationClass` "/Game/Objects/BP_AINav_Military.BP_AINav_Military_C"))))))
    (:`then_1`
      (bind _returnvalue (`|GenericCreateObject` (`local.AINavigationClass`)))
      (bind _output_get (set `self.AINavigation` _returnvalue))
      (`/Game/Objects/BP_AINav_Base.Setup` _output_get self))))