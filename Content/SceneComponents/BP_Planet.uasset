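; BP_Planet is a mesh component representing a planet in a campaign solar system, configured by its PlanetData.
; On BeginPlay it creates a dynamic material instance and tints it with the color of the planet's owning faction, looked up through the HUD's gamemode.
; It exposes location and radius through navigatable-style functions.
; DestroyNavigatable removes it from the solar system's clickable and planet lists, then destroys the component.
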(event `self.ReceiveBeginPlay`
  (bind _returnvalue (`self.CreateDynamicMaterialInstance` 0 (`self.GetMaterial` self 0)))
  (`MaterialInstanceDynamic.SetVectorParameterValue` _returnvalue "Color" (`KismetMathLibrary.Conv_ColorToLinearColor` (`/Game/FunctionLibraries/FL_Factions.GetFactionColor` (`.Faction_6_638D18E648A6E05053183A8AD8098D94` (break `/Game/Structs/S_PlanetData` (`self.PlanetData`))) (`/Game/Game/BP_HUD.Gamemode` (`/Game/ActorComponents/BP_CampaignManager.HUD` (`/Game/Actors/BP_SolarSystem.CampaignManager` (`self.SolarSystem`))))))))

(event `/Game/Interfaces/BI_NavigationSelectable.DestroyNavigatable`
  (bind _solarsystem (`self.SolarSystem`))
  (`KismetArrayLibrary.Array_RemoveItem` (`/Game/Actors/BP_SolarSystem.Clickables` _solarsystem) self)
  (`KismetArrayLibrary.Array_RemoveItem` (`/Game/Actors/BP_SolarSystem.Planets` _solarsystem) self)
  (`self.K2_DestroyComponent`))

(fn `GetAttachableComponent`
  (returns (Component :type "SceneComponent Object Reference"))
  (return null))

(fn `GetLocation`
  (returns (Location :type "Vector Structure"))
  (return (`self.K2_GetComponentLocation`)))

(fn `GetRadius`
  (returns (Radius :type "Float (double-precision)"))
  (return (`.Radius_29_418E822E486206A1739E309FE4EA9317` (break `/Game/Structs/S_PlanetData` (`self.PlanetData`)))))