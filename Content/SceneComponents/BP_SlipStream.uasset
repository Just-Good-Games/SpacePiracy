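; Scene component for a one-way slipstream that carries fleets from a start solar system to an end system.
; It registers fleets that reach it, then checks each tick for 2D circle overlap at the end location to release them into the end system.
; Debug arrows draw the path, with an entrance circle while the player is in the start system.
; Destruction removes it from the start system's lists.
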(event `self.ReceiveBeginPlay`
  (bind _output_get (set `self.StartLocation` (`self.K2_GetComponentLocation`)))
  (set `self.MiddleLocation` (/ (+ _output_get (`self.EndLocation`)) 2.0))
  (set `self.UnitDirection` (`KismetMathLibrary.GetDirectionUnitVector` (`self.StartLocation`) (`self.EndLocation`))))

(event `self.ReceiveTick`
  (params (DeltaSeconds :type "Float (single-precision)"))
  (bind _startsystem (`self.StartSystem`))
  (`KismetSystemLibrary.DrawDebugArrow` (`self.StartLocation`) (`self.MiddleLocation`) 10000000.0 (struct :`R` 1.0 :`G` 1.0 :`B` 1.0 :`A` 1.0))
  (`KismetSystemLibrary.DrawDebugArrow` (`self.MiddleLocation`) (`self.EndLocation`) 10000000.0 (struct :`R` 1.0 :`G` 1.0 :`B` 1.0 :`A` 1.0))
  (`self.CheckForFleetsLeaving`)
  (`/Engine/EditorBlueprintResources/StandardMacros.IsValid` _startsystem
    (:`Is Valid`
      (if (`/Game/Actors/BP_SolarSystem.ContainsPlayer` _startsystem)
        (`KismetSystemLibrary.DrawDebugCircle` (`self.StartLocation`) (`self.Radius`) 8 (struct :`R` 1.0 :`G` 1.0 :`B` 1.0 :`A` 1.0) 0.0 0.0 (0.0 1.0 0.0) (1.0 0.0 0.0))))))

(event `/Game/Interfaces/BI_NavigationSelectable.DestroyNavigatable`
  (bind _startsystem (`self.StartSystem`))
  (`KismetArrayLibrary.Array_RemoveItem` (`/Game/Actors/BP_SolarSystem.Clickables` _startsystem) self)
  (`KismetArrayLibrary.Array_RemoveItem` (`/Game/Actors/BP_SolarSystem.SlipSteams` _startsystem) self)
  (`self.K2_DestroyComponent`))

(fn `CheckForFleetsLeaving`
  (locals (TempFleets :type "Array of /Game/Actors/BP_CampaignFleet Object Reference"))
  (bind _output_get (set `local.TempFleets` (`self.Fleets`)))
  (for _array_element _output_get
    (`/Engine/EditorBlueprintResources/StandardMacros.IsValid` _array_element
      (:`Is Valid`
        (bind _radius (`/Game/Interfaces/BI_NavigationSelectable.GetRadius` _array_element))
        (bind _location (`/Game/Interfaces/BI_NavigationSelectable.GetLocation` _array_element))
        (bind _radius_2 (`/Game/Interfaces/BI_NavigationSelectable.GetRadius` self))
        (bind _bcollision (`/JGGUniversalFunctionsAndMacros/FunctionLibraries/FL_Transformation.SimpleCircleCollisionCheck2D` (`self.EndLocation`) _radius_2 _location _radius))
        (if _bcollision
          (set `/Game/Actors/BP_CampaignFleet.SlipStream` null _array_element)
          (`KismetArrayLibrary.Array_RemoveItem` (`self.Fleets`) _array_element)
          (`/Game/Actors/BP_CampaignFleet.UpdateFleetLocation` _array_element (`self.EndLocation`))
          (`/Game/Actors/BP_CampaignFleet.ChangeSolarSystem` _array_element (`self.EndSystem`)))))))

(fn `GetAttachableComponent`
  (returns (Component :type "SceneComponent Object Reference"))
  (return null))

(fn `GetLocation`
  (returns (Location :type "Vector Structure"))
  (return (`self.K2_GetComponentLocation`)))

(fn `GetRadius`
  (returns (Radius :type "Float (double-precision)"))
  (return (`self.Radius`)))

(fn `GetVelocityIfAny`
  (returns (Velocity :type "Vector Structure"))
  (return (0.0 0.0 0.0)))

(fn `OnFleetReached`
  (params (Fleet :type "/Game/Actors/BP_CampaignFleet Object Reference"))
  (`KismetArrayLibrary.Array_Add` (`self.Fleets`) Fleet))