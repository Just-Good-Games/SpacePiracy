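; BP_TutorialDestination is a mesh component that marks a navigation destination for the player in the tutorial, tinted yellow through a dynamic material instance at BeginPlay.
; It exposes its world location and radius to navigation, and returns no attachable component.
; When the player reaches it, it fires PlayerReached and destroys itself.
; DestroyNavigatable instead removes it from the SolarSystem's Clickables before destroying it.
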(event `self.ReceiveBeginPlay`
  (bind _returnvalue (`self.CreateDynamicMaterialInstance` 0 (`self.GetMaterial` self 0)))
  (`MaterialInstanceDynamic.SetVectorParameterValue` _returnvalue "Color" (struct :`R` 1.0 :`G` 1.0 :`A` 1.0)))

(event `/Game/Interfaces/BI_NavigationSelectable.DestroyNavigatable`
  (`KismetArrayLibrary.Array_RemoveItem` (`/Game/Actors/BP_SolarSystem.Clickables` (`self.SolarSystem`)) self)
  (`self.K2_DestroyComponent`))

(fn `GetAttachableComponent`
  (returns (Component :type "SceneComponent Object Reference"))
  (return null))

(fn `GetLocation`
  (returns (Location :type "Vector Structure"))
  (return (`self.K2_GetComponentLocation`)))

(fn `GetRadius`
  (returns (Radius :type "Float (double-precision)"))
  (return (`self.Radius`)))

(fn `OnPlayerReached`
  (`self.PlayerReached`)
  (`self.K2_DestroyComponent`))