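; BP_TutorialAIDestination is a scene component that acts as a navigatable destination point, named for AI use in the tutorial.
; It answers navigation queries with its world location, zero velocity, no attachable component, and the default radius of BP_SlipStream.
; DestroyNavigatable removes it from the SolarSystem's Unclickables list when that system is valid, then destroys the component.
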(event `self.ReceiveBeginPlay`)

(event `self.ReceiveTick`
  (params (DeltaSeconds :type "Float (single-precision)")))

(event `self.DestroyNavigatable`
  (bind _solarsystem (`self.SolarSystem`))
  (`/Engine/EditorBlueprintResources/StandardMacros.IsValid` _solarsystem
    (:`Is Valid`
      (`KismetArrayLibrary.Array_RemoveItem` (`/Game/Actors/BP_SolarSystem.Unclickables` _solarsystem) self))
    (:`Is Not Valid`
      _))
  (`self.K2_DestroyComponent`))

(fn `GetAttachableComponent`
  (returns (Component :type "SceneComponent Object Reference"))
  (return null))

(fn `GetLocation`
  (returns (Location :type "Vector Structure"))
  (return (`self.K2_GetComponentLocation`)))

(fn `GetRadius`
  (returns (Radius :type "Float (double-precision)"))
  (return (`.Radius` (defaults `/Game/SceneComponents/BP_SlipStream` "/Game/SceneComponents/BP_SlipStream.BP_SlipStream_C"))))

(fn `GetVelocityIfAny`
  (returns (Velocity :type "Vector Structure"))
  (return (0.0 0.0 0.0)))