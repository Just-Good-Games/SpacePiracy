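; Actor component for a fleet that owns ship components, aggregate ship stats and per-faction bounty records.
; A data table template fills a queue submitted to BP_GameMode, and CreateQueuedShip spawns one ship per call.
; Captured ships stay pending until finalized, joining only on a win.
; Crimes add bounty with the target and influence with Pirates, while other factions gain favor as negative bounty, which can decay.
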(event `self.ReceiveBeginPlay`
  (if (`self.bAutomaticSetup`)
    (`self.CreateShipsFromFleetTemplate`)))

(fn `AddRemoveShip`
  (params (Ship :type "/Game/ActorComponents/BP_Ship Object Reference") (bAdding :type Boolean))
  (bind _ships (`self.Ships`))
  (bind _ship (`local.Ship`))
  (`|ExecutionSequence`
    (:`then_0`
      (bind _keys (`BlueprintMapLibrary.Map_Keys` (`self.FleetStats`)))
      (for _array_element _keys
        (bind (_value _returnvalue) (`BlueprintMapLibrary.Map_Find` (`/Game/ActorComponents/BP_Ship.ShipStats` (`local.Ship`)) _array_element))
        (if _returnvalue
          (`/JGGUniversalFunctionsAndMacros/Macros/BM_Maps.IncrementIntegerMap` (`self.FleetStats`) _array_element (* _value (select `bool` bAdding :`false` -1 :`true` 1))))))
    (:`then_1`
      (if bAdding
        (`KismetArrayLibrary.Array_Add` _ships _ship)
        (set `/Game/ActorComponents/BP_Ship.Fleet` self _ship)
        (else
          (`KismetArrayLibrary.Array_RemoveItem` _ships _ship)
          (set `/Game/ActorComponents/BP_Ship.Fleet` null _ship))))))

(fn `AddShipCaptures`
  (bind _capturedships (`self.CapturedShips`))
  (for _array_element _capturedships
    (`/Game/ActorComponents/BP_Ship.ChangeFleet` _array_element self))
  (`KismetArrayLibrary.Array_Clear` _capturedships))

(fn `CheckIfFleetIsDestroyed`
  (if (`KismetArrayLibrary.Array_IsEmpty` (`self.Ships`))
    (`self.OnFleetDestroyed`)))

(fn `CreateQueuedShip`
  (returns (FleetFinished :type Boolean))
  (bind _shiptemplatesqueue (`self.ShipTemplatesQueue`))
  (bind _returnvalue (`|AddComponentByClass` (`self.GetOwner`) "/Game/ActorComponents/BP_Ship.BP_Ship_C" (`|GetArrayItem` (`self.ShipTemplatesQueue`)) (`self.FleetType`) self))
  (`KismetArrayLibrary.Array_Add` (`self.Ships`) _returnvalue)
  (`KismetArrayLibrary.Array_Remove` _shiptemplatesqueue)
  (if (<= (`KismetArrayLibrary.Array_Length` _shiptemplatesqueue) 0)
    (`self.FinishedSettingupTemplates`)
    (return true)
    (else
      (return false))))

(fn `CreateShipsFromFleetTemplate`
  (locals (FleetTemplateTable :type "DataTable Object Reference" :default "/Script/Engine.DataTable'/Game/DataTables/DT_FleetTemplates.DT_FleetTemplates'"))
  (`self.ResetTemplate`)
  (bind _returnvalue (`|GetDataTableRow` (`local.FleetTemplateTable`) (`self.FleetTemplate`))
    (:`then`
      (bind (_fleettype _shiptemplates _money) (break `/Game/Structs/S_FleetTemplate` _returnvalue))
      (set `self.FleetType` _fleettype)
      (set `self.Money` _money)
      (bind _keys (`BlueprintMapLibrary.Map_Keys` _shiptemplates))
      (for _array_element _keys
        (bind (_value _returnvalue_2) (`BlueprintMapLibrary.Map_Find` _shiptemplates _array_element))
        (if _returnvalue_2
          (for _ (range 1 (+ _value 1))
            (`KismetArrayLibrary.Array_Add` (`self.ShipTemplatesQueue`) _array_element))))
      (bind _asbp_game_mode (cast `/Game/Game/BP_GameMode` (`GameplayStatics.GetGameMode`)))
      (`/Game/Game/BP_GameMode.QueueFleet` _asbp_game_mode self))))

(fn `DecayAllFactionFavor`
  (locals (Factions :type "Array of /Game/GlobalEnums/E_Faction Enum"))
  (for _array_element (`local.Factions`)
    (`self.DecayFactionFavor` _array_element)))

(fn `DecayFactionFavor`
  (params (Faction :type "/Game/GlobalEnums/E_Faction Enum" :default "NewEnumerator0"))
  (locals (ResetFactionFavorAmount :type Integer :default 0) (RemianingProportion :type "Float (double-precision)" :default 0.9))
  (bind _factionbounty (`self.GetFactionBountyStats` Faction))
  (bind (_value _returnvalue) (`BlueprintMapLibrary.Map_Find` _factionbounty "NewEnumerator7"))
  (bind _returnvalue_2 (`KismetMathLibrary.FTrunc` (* _value (`local.RemianingProportion`))))
  (if _returnvalue
    (if (>= _returnvalue_2 (`local.ResetFactionFavorAmount`))
      (`BlueprintMapLibrary.Map_Remove` _factionbounty "NewEnumerator7")
      (else
        (`BlueprintMapLibrary.Map_Add` _factionbounty "NewEnumerator7" _returnvalue_2)))))

(fn `FinalizeShipCaptures`
  (params (bWon :type Boolean))
  (if bWon
    (`self.AddShipCaptures`)
    (else
      (`self.UndoShipCaptures`))))

(fn `GetFactionBountyAmount`
  (params (Faction :type "/Game/GlobalEnums/E_Faction Enum" :default "NewEnumerator0"))
  (returns (Bounty :type Integer))
  (locals (BountyStats :type "Map of /Game/GlobalEnums/E_Crimes Enum to Integer") (TotalBounty :type Integer))
  (bind _output_get (set `local.BountyStats` (`self.GetFactionBountyStats` Faction)))
  (bind _keys (`BlueprintMapLibrary.Map_Keys` _output_get))
  (for _array_element _keys
    (bind (_value _returnvalue) (`BlueprintMapLibrary.Map_Find` _output_get _array_element))
    (if _returnvalue
      (set `local.TotalBounty` (+ (`local.TotalBounty`) _value))))
  (return (`local.TotalBounty`)))

(fn `GetFactionBountyStats`
  (params (Faction :type "/Game/GlobalEnums/E_Faction Enum" :default "NewEnumerator0"))
  (returns (FactionBounty :type "Map of /Game/GlobalEnums/E_Crimes Enum to Integer"))
  (return (select `/Game/GlobalEnums/E_Faction` Faction :`NewEnumerator5` (`self.PirateInfluence`) :`NewEnumerator4` (`self.YellowBounty`) :`NewEnumerator3` (`self.GreenBounty`) :`NewEnumerator2` (`self.BlueBounty`) :`NewEnumerator1` (`self.RedBounty`))))

(fn `GetFleetStats`
  (params (Stat :type "/Game/GlobalEnums/E_TradeGoodProperty Enum" :default "NewEnumerator0"))
  (returns (Value :type Integer))
  (bind (_value _returnvalue) (`BlueprintMapLibrary.Map_Find` (`self.FleetStats`) Stat))
  (if _returnvalue
    (return _value)
    (else
      (return 0))))

(fn `RecordCrimeCommitted`
  (params (TargetFaction :type "/Game/GlobalEnums/E_Faction Enum" :default "NewEnumerator0") (Crime :type "/Game/GlobalEnums/E_Crimes Enum" :default "NewEnumerator0") (Bounty :type Integer))
  (locals (Factions :type "Array of /Game/GlobalEnums/E_Faction Enum"))
  (for _array_element (`local.Factions`)
    (`self.RecordFactionReactionToCrime` _array_element TargetFaction Crime Bounty)))

(fn `RecordFactionReactionToCrime`
  (params (ReactingFaction :type "/Game/GlobalEnums/E_Faction Enum" :default "NewEnumerator0") (TargetFaction :type "/Game/GlobalEnums/E_Faction Enum" :default "NewEnumerator0") (Crime :type "/Game/GlobalEnums/E_Crimes Enum" :default "NewEnumerator0") (Bounty :type Integer))
  (locals (bApproves :type Boolean))
  (bind _bounty (`local.Bounty`))
  (set `local.bApproves` (and (`|EnumInequality` ReactingFaction TargetFaction) (`|EnumInequality` ReactingFaction "NewEnumerator5")))
  (`/JGGUniversalFunctionsAndMacros/Macros/BM_Maps.IncrementIntegerMap` (`self.GetFactionBountyStats` (`local.ReactingFaction`)) (select `bool` (`local.bApproves`) :`false` (`local.Crime`) :`true` "NewEnumerator7") (select `bool` (`local.bApproves`) :`false` _bounty :`true` (* _bounty -1))))

(fn `ResetTemplate`
  (`|ExecutionSequence`
    (:`then_0`
      (for _array_element (`self.Ships`)
        (`self.K2_DestroyComponent` _array_element)))
    (:`then_1`
      (`KismetArrayLibrary.Array_Clear` (`self.Ships`))
      (`BlueprintMapLibrary.Map_Clear` (`self.FleetStats`)))))

(fn `TemporaryCaptureShip`
  (params (Ship :type "/Game/ActorComponents/BP_Ship Object Reference"))
  (`KismetArrayLibrary.Array_Add` (`self.CapturedShips`) Ship))

(fn `UndoShipCaptures`
  (`KismetArrayLibrary.Array_Clear` (`self.CapturedShips`)))