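; Ship actor component within a fleet, built from a data table template with deployed, destroyed and stored components.
; Component changes check slots and power, then update ship and fleet stat totals.
; Battle stats derive from ship stats, absorb damage in per-target cascade order, then convert post-battle losses into destroyed components.
; It also supplies combat rolls, takes target and strategy from player UI or fixed AI choices, and handles fleet transfer and destruction.
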(event `self.ReceiveBeginPlay`
  (`self.CreateShipFromTemplate`))

(fn `ApplyBattleDamage`
  (params (Target :type "/Game/GlobalEnums/E_BattleTarget Enum" :default "NewEnumerator0") (Damage :type Integer))
  (returns (Result :type "/Game/GlobalEnums/E_BattleResult Enum"))
  (locals (EngineFocusTargetOrder :type "Array of /Game/GlobalEnums/E_BattleTarget Enum") (ShieldFocusTargetOrder :type "Array of /Game/GlobalEnums/E_BattleTarget Enum") (GunFocusTargetOrder :type "Array of /Game/GlobalEnums/E_BattleTarget Enum") (KillFocusTargetOrder :type "Array of /Game/GlobalEnums/E_BattleTarget Enum") (CurrentDamage :type Integer))
  (bind _output_get (set `local.CurrentDamage` Damage))
  (if (> _output_get 0)
    (for _array_element (select `/Game/GlobalEnums/E_BattleTarget` Target :`NewEnumerator1` (`local.EngineFocusTargetOrder`) :`NewEnumerator2` (`local.ShieldFocusTargetOrder`) :`NewEnumerator3` (`local.GunFocusTargetOrder`) :`NewEnumerator4` (`local.KillFocusTargetOrder`))
      (bind (_remainingdamage _bdestroyedtarget) (`self.ApplyBattleDamageInternal` _array_element (`local.CurrentDamage`)))
      (set `local.CurrentDamage` _remainingdamage)
      (if (not _bdestroyedtarget)
        (return "NewEnumerator1")))
    (return (select `/Game/GlobalEnums/E_BattleTarget` (`local.Target`) :`NewEnumerator0` "NewEnumerator0" :`NewEnumerator1` "NewEnumerator2" :`NewEnumerator2` "NewEnumerator2" :`NewEnumerator3` "NewEnumerator2" :`NewEnumerator4` "NewEnumerator3" :`NewEnumerator5` "NewEnumerator0" :!type "/Game/GlobalEnums/E_BattleResult Enum"))
    (else
      (return "NewEnumerator1"))))

(fn `ApplyBattleDamageInternal`
  (params (BattleTarget :type "/Game/GlobalEnums/E_BattleTarget Enum" :default "NewEnumerator0") (Damage :type Integer))
  (returns (RemainingDamage :type Integer) (bDestroyedTarget :type Boolean))
  (locals (NewValue :type Integer))
  (bind _battlestats (`self.BattleStats`))
  (bind _battletarget (`local.BattleTarget`))
  (set `local.NewValue` (- (`BlueprintMapLibrary.Map_Find` (`self.BattleStats`) BattleTarget) Damage))
  (`BlueprintMapLibrary.Map_Remove` (`self.BattleStats`) (`local.BattleTarget`))
  (if (<= (`local.NewValue`) 0)
    (`BlueprintMapLibrary.Map_Add` _battlestats _battletarget)
    (return (`KismetMathLibrary.Abs_Int` (`local.NewValue`)) true)
    (else
      (`BlueprintMapLibrary.Map_Add` _battlestats _battletarget (`local.NewValue`))
      (return 0 false))))

(fn `ApplyPostBattleDamage`
  (`self.CalculateStatChangeFromDamage`)
  (`self.DestroyComponentsFromStatChange`))

(fn `CalculateBattleStats`
  (bind _battlestats (`self.BattleStats`))
  (`BlueprintMapLibrary.Map_Clear` _battlestats)
  (`BlueprintMapLibrary.Map_Add` _battlestats "NewEnumerator1" (`KismetMathLibrary.FCeil` (/ (`KismetMathLibrary.Conv_IntToDouble` (`self.GetShipStat` "NewEnumerator9")) (`KismetMathLibrary.Conv_IntToDouble` (`self.GetShipStat` "NewEnumerator1")))))
  (`BlueprintMapLibrary.Map_Add` _battlestats "NewEnumerator2" (`self.GetShipStat` "NewEnumerator8"))
  (`BlueprintMapLibrary.Map_Add` _battlestats "NewEnumerator3" (`self.GetShipStat` "NewEnumerator7"))
  (`BlueprintMapLibrary.Map_Add` _battlestats "NewEnumerator5" (`self.GetShipStat` "NewEnumerator6"))
  (`BlueprintMapLibrary.Map_Add` _battlestats "NewEnumerator4" (`KismetMathLibrary.FCeil` (/ (`KismetMathLibrary.Conv_IntToDouble` (`self.GetShipStat` "NewEnumerator10")) (`KismetMathLibrary.Conv_IntToDouble` (`self.GetShipStat` "NewEnumerator3")))))
  (set `self.PreBattleStats` (`self.BattleStats`)))

(fn `CalculateStatChangeFromDamage`
  (`BlueprintMapLibrary.Map_Clear` (`self.DamagedStats`))
  (`BlueprintMapLibrary.Map_Add` (`self.DamagedStats`) "NewEnumerator9" (* (`BlueprintMapLibrary.Map_Find` (`self.BattleStats`) "NewEnumerator1") (`self.GetShipStat` "NewEnumerator1")))
  (`BlueprintMapLibrary.Map_Add` (`self.DamagedStats`) "NewEnumerator8" (`BlueprintMapLibrary.Map_Find` (`self.BattleStats`) "NewEnumerator2"))
  (`BlueprintMapLibrary.Map_Add` (`self.DamagedStats`) "NewEnumerator7" (`BlueprintMapLibrary.Map_Find` (`self.BattleStats`) "NewEnumerator3"))
  (`BlueprintMapLibrary.Map_Add` (`self.DamagedStats`) "NewEnumerator6" (`BlueprintMapLibrary.Map_Find` (`self.BattleStats`) "NewEnumerator5"))
  (`BlueprintMapLibrary.Map_Add` (`self.DamagedStats`) "NewEnumerator9" (* (`BlueprintMapLibrary.Map_Find` (`self.BattleStats`) "NewEnumerator4") (`self.GetShipStat` "NewEnumerator3"))))

(fn `ChangeComponents`
  (params (ShipComponent :type "/Game/Structs/S_ShipComponent Structure") (ChangeNumber :type Integer) (State :type "/Game/GlobalEnums/E_ShipComponentState Enum" :default "NewEnumerator0") (bIgnorePowerRequirement :type Boolean :default false))
  (returns (bSuccess :type Boolean))
  (bind _changenumber (`local.ChangeNumber`))
  (bind _freearmourslots (`self.FreeArmourSlots`))
  (bind _shipcomponent (`local.ShipComponent`))
  (bind (_tradegood _rank) (break `/Game/Structs/S_ShipComponent` (`local.ShipComponent`)))
  (bind _returnvalue (select `/Game/GlobalEnums/E_ShipComponentState` State :`NewEnumerator1` (`self.DeployedComponents`) :`NewEnumerator2` (`self.DestroyedComponents`) :`NewEnumerator3` (`self.StoredComponents`)))
  (bind (_value _returnvalue_2) (`BlueprintMapLibrary.Map_Find` _returnvalue (`local.ShipComponent`)))
  (bind _type (`/Game/FunctionLibraries/FL_TradeGoods.GetTradeGoodType` (`.TradeGood_2_520825BF4FF280580CE275961ED246F2` (break `/Game/Structs/S_ShipComponent` (`local.ShipComponent`)))))
  (if (and (`|EnumInequality` State "NewEnumerator0") (!= ChangeNumber 0))
    (if (> (`local.ChangeNumber`) 0)
      (if (>= (select `/Game/GlobalEnums/E_TradeGoodType` _type :`NewEnumerator2` (select `/Game/GlobalEnums/E_ShipComponentState` (`local.State`) :`NewEnumerator1` _freearmourslots :`NewEnumerator2` _freearmourslots :`NewEnumerator3` (`self.FreeCargoSlots`)) :`NewEnumerator3` (`self.FreeCargoSlots`)) (* (select `/Game/GlobalEnums/E_TradeGoodType` _type :`NewEnumerator2` 1 :`NewEnumerator3` (select `/Game/GlobalEnums/E_ShipComponentState` (`local.State`) :`NewEnumerator1` 2 :`NewEnumerator2` 2 :`NewEnumerator3` 1)) (`local.ChangeNumber`)))
        (if (or (>= (+ (* (`/Game/FunctionLibraries/FL_TradeGoods.GetTradeGoodProperty` _tradegood "NewEnumerator5" (`local.State`) _rank) (`local.ChangeNumber`)) (`self.GetShipStat` "NewEnumerator5")) 0) (`local.bIgnorePowerRequirement`))
          _
          (else
            (return false)))
        (else
          (return false)))
      (elif (and _returnvalue_2 (>= _value (* (`local.ChangeNumber`) -1)))
        _
        (else
          (return false))))
    (`/JGGUniversalFunctionsAndMacros/Macros/BM_Maps.IncrementIntegerMap` _returnvalue _shipcomponent _changenumber
      (:`OutExec`
        (`self.ChangeShipStats` _shipcomponent _changenumber (`local.State`))
        (return true)))
    (else
      (return false))))

(fn `ChangeFleet`
  (params (NewFleet :type "/Game/ActorComponents/BP_Fleet Object Reference"))
  (`/Game/ActorComponents/BP_Fleet.AddRemoveShip` (`self.Fleet`) self false)
  (`/Game/ActorComponents/BP_Fleet.AddRemoveShip` (`local.NewFleet`) self true))

(fn `ChangeShipStats`
  (params (ShipComponent :type "/Game/Structs/S_ShipComponent Structure") (Change :type Integer) (State :type "/Game/GlobalEnums/E_ShipComponentState Enum" :default "NewEnumerator0"))
  (locals (StatChange :type Integer))
  (bind (_tradegood _rank) (break `/Game/Structs/S_ShipComponent` ShipComponent))
  (for _array_element (`/Game/FunctionLibraries/FL_TradeGoods.GetTradeGoodProperties` _tradegood)
    (bind _output_get (set `local.StatChange` (* (`/Game/FunctionLibraries/FL_TradeGoods.GetTradeGoodProperty` _tradegood _array_element (`local.State`) _rank) (`local.Change`))))
    (`/JGGUniversalFunctionsAndMacros/Macros/BM_Maps.IncrementIntegerMap` (`self.ShipStats`) _array_element _output_get
      (:`OutExec`
        (`/JGGUniversalFunctionsAndMacros/Macros/BM_Maps.IncrementIntegerMap` (`/Game/ActorComponents/BP_Fleet.FleetStats` (`self.Fleet`)) _array_element (`local.StatChange`)
          (:`OutExec`
            (`/JGGErrorAndTesting/FunctionLibraries/FL_Error.PrintMessage` self "NewEnumerator0" (`KismetStringLibrary.Concat_StrStr` (`|GetEnumeratorNameAsString` _tradegood) " - " (`|GetEnumeratorNameAsString` _array_element) " changed by " (`KismetStringLibrary.Conv_IntToString` (`local.StatChange`)) " to " (`KismetStringLibrary.Conv_IntToString` 0)) "None" true))))))
  (switch `/Game/GlobalEnums/E_TradeGoodType` (`/Game/FunctionLibraries/FL_TradeGoods.GetTradeGoodType` _tradegood)
    (:`NewEnumerator1`
      (set `self.FreeCargoSlots` (`self.GetShipStat` "NewEnumerator4"))
      (set `self.FreeArmourSlots` (`self.GetShipStat` "NewEnumerator3")))
    (:`NewEnumerator2`
      (if (select `/Game/GlobalEnums/E_ShipComponentState` (`local.State`) :`NewEnumerator1` true :`NewEnumerator2` true)
        (set `self.FreeArmourSlots` (+ (* (`local.Change`) -1) (`self.FreeArmourSlots`)))
        (else
          (set `self.FreeCargoSlots` (+ (* (`local.Change`) (select `/Game/GlobalEnums/E_ShipComponentState` (`local.State`) :`NewEnumerator1` 2 :`NewEnumerator2` 2 :`NewEnumerator3` 1) -1) (`self.FreeCargoSlots`)) :!label _label))))
    (:`NewEnumerator3`
      (goto _label))))

(fn `CreateComponentsOfStateFromTemplate`
  (params (Components :type "Map of /Game/GlobalEnums/E_TradeGood Enum to Integer") (State :type "/Game/GlobalEnums/E_ShipComponentState Enum" :default "NewEnumerator0"))
  (if (`|EnumInequality` State "NewEnumerator0")
    (bind _keys (`BlueprintMapLibrary.Map_Keys` Components))
    (for _array_element _keys
      (bind (_value _returnvalue) (`BlueprintMapLibrary.Map_Find` Components _array_element))
      (if _returnvalue
        (`self.ChangeComponents` (make `/Game/Structs/S_ShipComponent` _array_element 1) _value State true)))))

(fn `CreateShipFromTemplate`
  (locals (ShipTemplateTable :type "DataTable Object Reference" :default "/Script/Engine.DataTable'/Game/DataTables/DT_ShipTemplates.DT_ShipTemplates'"))
  (bind _value (`self.GetShipStat` "NewEnumerator5"))
  (bind _returnvalue (`|GetDataTableRow` (`local.ShipTemplateTable`) (`self.ShipTemplate`))
    (:`then`
      (bind (_shiptype _deployedcomponents _destroyedcomponents _storedcomponents) (break `/Game/Structs/S_ShipTemplate` _returnvalue))
      (bind _output_get (set `self.ShipType` _shiptype))
      (`self.ChangeShipStats` (make `/Game/Structs/S_ShipComponent` _output_get 1) 1 "NewEnumerator1")
      (`self.CreateComponentsOfStateFromTemplate` _deployedcomponents "NewEnumerator1")
      (`self.CreateComponentsOfStateFromTemplate` _destroyedcomponents "NewEnumerator2")
      (`self.CreateComponentsOfStateFromTemplate` _storedcomponents "NewEnumerator3")
      (if (< _value 0)
        (`/JGGErrorAndTesting/FunctionLibraries/FL_Error.PrintMessage` self "NewEnumerator1" (`KismetStringLibrary.Concat_StrStr` (`KismetStringLibrary.Conv_NameToString` (`self.ShipTemplate`)) " template has negative power = " (`KismetStringLibrary.Conv_IntToString` _value)))))))

(fn `DestroyComponentsFromStatChange`
  (locals (Components :type "Array of /Game/Structs/S_ShipComponent Structure"))
  (bind _keys (`BlueprintMapLibrary.Map_Keys` (`self.DeployedComponents`)))
  (bind _output_get (set `local.Components` _keys))
  (for _array_element _output_get
    (bind (_tradegood _rank) (break `/Game/Structs/S_ShipComponent` _array_element))
    (for _array_element_2 (`/Game/FunctionLibraries/FL_TradeGoods.GetTradeGoodProperties` _tradegood)
      (bind (_value _returnvalue) (`BlueprintMapLibrary.Map_Find` (`self.DeployedComponents`) _array_element))
      (bind (_value_2 _returnvalue_2) (`BlueprintMapLibrary.Map_Find` (`self.ShipStats`) _array_element_2))
      (bind (_value_3 _returnvalue_3) (`BlueprintMapLibrary.Map_Find` (`self.DamagedStats`) _array_element_2))
      (if (and _returnvalue _returnvalue_2 _returnvalue_3)
        (bind _returnvalue_4 (- _value_2 _value_3))
        (if (> _returnvalue_4 0)
          (bind _returnvalue_5 (`KismetMathLibrary.Min` _value (`KismetMathLibrary.Round` (`KismetMathLibrary.SafeDivide` (`KismetMathLibrary.Conv_IntToDouble` _returnvalue_4) (`KismetMathLibrary.Conv_IntToDouble` (`/Game/FunctionLibraries/FL_TradeGoods.GetTradeGoodProperty` _tradegood _array_element_2 "NewEnumerator1" _rank))))))
          (bind _bsuccess (`self.ChangeComponents` _array_element (* _returnvalue_5 -1) "NewEnumerator1"))
          (if _bsuccess
            (`self.ChangeComponents` _array_element _returnvalue_5 "NewEnumerator2")))))))

(fn `DestroyShip`
  (bind _fleet (`self.Fleet`))
  (bind _keys (`BlueprintMapLibrary.Map_Keys` (`self.ShipStats`)))
  (for _array_element _keys
    (`/JGGUniversalFunctionsAndMacros/Macros/BM_Maps.IncrementIntegerMap` (`/Game/ActorComponents/BP_Fleet.FleetStats` (`self.Fleet`)) _array_element (* (`BlueprintMapLibrary.Map_Find` (`self.ShipStats`) _array_element) -1)))
  (`KismetArrayLibrary.Array_RemoveItem` (`/Game/ActorComponents/BP_Fleet.Ships` _fleet) self)
  (`self.K2_DestroyComponent` self)
  (`/Game/ActorComponents/BP_Fleet.CheckIfFleetIsDestroyed` _fleet))

(fn `GetBattleStat`
  (params (Stat :type "/Game/GlobalEnums/E_BattleTarget Enum" :default "NewEnumerator0"))
  (returns (Value :type Integer))
  (bind (_value _returnvalue) (`BlueprintMapLibrary.Map_Find` (`self.BattleStats`) Stat))
  (if _returnvalue
    (return _value)
    (else
      (return 0))))

(fn `GetBattleStatAlternateZeroCalc`
  (params (Stat :type "/Game/GlobalEnums/E_BattleTarget Enum" :default "NewEnumerator0"))
  (returns (bAlternateZeroCalculation :type Boolean))
  (return (select `/Game/GlobalEnums/E_BattleTarget` Stat :`NewEnumerator1` true)))

(fn `GetBattleStatRoll`
  (params (Stat :type "/Game/GlobalEnums/E_BattleTarget Enum" :default "NewEnumerator0"))
  (returns (Value :type Integer))
  (return (`/Game/FunctionLibraries/FL_ProbabilityCalculator.RandomRoll` (`self.GetBattleStat` Stat) (`self.GetBattleStatAlternateZeroCalc` Stat))))

(fn `GetBattleStrategy`
  (returns (Target :type "/Game/GlobalEnums/E_BattleStrategy Enum"))
  (if (`/Game/ActorComponents/BP_Fleet.bIsPlayer` (`self.Fleet`))
    (return (`self.GetBattleStrategyPlayer`))
    (else
      (return (`self.GetBattleStrategyComputer`)))))

(fn `GetBattleStrategyComputer`
  (returns (Target :type "/Game/GlobalEnums/E_BattleStrategy Enum"))
  (return "NewEnumerator1"))

(fn `GetBattleStrategyPlayer`
  (returns (Strategy :type "/Game/GlobalEnums/E_BattleStrategy Enum"))
  (return (`/Game/Widgets/Battle/WB_BattleUI.PlayerStrategy` (`/Game/Game/BP_HUD.CombatUI` (`/Game/ActorComponents/BP_Fleet.Hud` (`self.Fleet`))))))

(fn `GetBattleTarget`
  (returns (Target :type "/Game/GlobalEnums/E_BattleTarget Enum"))
  (if (`/Game/ActorComponents/BP_Fleet.bIsPlayer` (`self.Fleet`))
    (return (`self.GetBattleTargetPlayer`))
    (else
      (return (`self.GetBattleTargetComputer`)))))

(fn `GetBattleTargetComputer`
  (returns (Target :type "/Game/GlobalEnums/E_BattleTarget Enum"))
  (locals (TargetOptions :type "Array of /Game/GlobalEnums/E_BattleTarget Enum"))
  (return "NewEnumerator4"))

(fn `GetBattleTargetPlayer`
  (returns (Target :type "/Game/GlobalEnums/E_BattleTarget Enum"))
  (return (`/Game/Widgets/Battle/WB_BattleUI.PlayerTarget` (`/Game/Game/BP_HUD.CombatUI` (`/Game/ActorComponents/BP_Fleet.Hud` (`self.Fleet`))))))

(fn `GetDamageRoll`
  (params (bHasAdvantage :type Boolean))
  (returns (Value :type Integer))
  (if bHasAdvantage
    (return (`self.GetManeuverAdvantageDamage`))
    (else
      (return (`self.GetBattleStatRoll` "NewEnumerator3")))))

(fn `GetManeuverAdvantageDamage`
  (returns (Value :type Integer))
  (return (`/Game/FunctionLibraries/FL_ProbabilityCalculator.RandomRoll` (+ (`self.GetBattleStat` "NewEnumerator3") (`self.GetBattleStat` "NewEnumerator5")))))

(fn `GetShipStat`
  (params (Stat :type "/Game/GlobalEnums/E_TradeGoodProperty Enum" :default "NewEnumerator0"))
  (returns (Value :type Integer))
  (bind (_value _returnvalue) (`BlueprintMapLibrary.Map_Find` (`self.ShipStats`) Stat))
  (if _returnvalue
    (return _value)
    (else
      (return 0))))