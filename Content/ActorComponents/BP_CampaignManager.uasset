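; BP_CampaignManager builds and tears down the galaxy map of solar systems for a campaign.
; Generation looks up the campaign's data table and spawns a BP_SolarSystem per row, converting its 2D position to world space within the galaxy radius.
; Spawned systems are tracked in a map by row name and can be dereferenced individually.
; Teardown destroys every system, restores the main menu UI and disables dialogue.
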(fn `DereferenceSolarSystem`
  (params (SolarSystem :type Name))
  (bind _returnvalue (`BlueprintMapLibrary.Map_Remove` (`self.SolarSystems`) SolarSystem)))

(fn `DestroyCampaignMap`
  (bind _hud (`self.HUD`))
  (bind _values (`BlueprintMapLibrary.Map_Values` (`self.SolarSystems`)))
  (for _array_element _values
    (`/Game/Actors/BP_SolarSystem.DestroySolarSystem` _array_element))
  (`Widget.SetVisibility` (`/Game/Game/BP_HUD.MainMenuUI` _hud) "Visible")
  (`Widget.SetVisibility` (`/Game/Game/BP_HUD.CampaignUI` _hud) "Hidden")
  (`/JGGUniversalFunctionsAndMacros/ActorComponenets/BP_DialogueComponent.DisableDialogue` (`/Game/Game/BP_GameMode.DialogueComponent` (`/Game/Game/BP_HUD.Gamemode` (`self.HUD`)))))

(fn `GenerateCampaignMap`
  (params (Campaign :type "/Game/GlobalEnums/E_Campaigns Enum" :default "NewEnumerator0") (bGenerateShips :type Boolean) (PlayerTemplate :type Name))
  (locals (CurrentSolarSystemTable :type "DataTable Object Reference") (SolarSystemTables :type "Map of /Game/GlobalEnums/E_Campaigns Enum to DataTable Object Reference") (GalaxyRadius :type "Float (double-precision)" :default 1000000.0))
  (bind (_value _returnvalue) (`BlueprintMapLibrary.Map_Find` (`local.SolarSystemTables`) Campaign))
  (set `self.CurrentPlayer` PlayerTemplate)
  (if _returnvalue
    (set `local.CurrentSolarSystemTable` _value)
    (bind _outrownames (`DataTableFunctionLibrary.GetDataTableRowNames` (`local.CurrentSolarSystemTable`)))
    (for _array_element _outrownames
      (bind _returnvalue_2 (`|GetDataTableRow` (`local.CurrentSolarSystemTable`) _array_element)
        (:`then`
          (bind _returnvalue_3 (`|SpawnActorFromClass` "/Game/Actors/BP_SolarSystem.BP_SolarSystem_C" (`/JGGUniversalFunctionsAndMacros/FunctionLibraries/FL_Transformation.Relative2DToWorldTransform3D` (0.0 0.0 0.0) (`.Position_53_9BD1623846C8C233090FD984EED15A45` (break `/Game/Structs/S_SolarSystemData` _returnvalue_2)) (`local.GalaxyRadius`)) "Undefined" "MultiplyWithRoot" null _returnvalue_2 (`local.bGenerateShips`) self _array_element null))
          (`BlueprintMapLibrary.Map_Add` (`self.SolarSystems`) _array_element _returnvalue_3))))
    (else
      (`/JGGErrorAndTesting/FunctionLibraries/FL_Error.PrintMessage` self "NewEnumerator1" (`KismetStringLibrary.Concat_StrStr` "Tried to load an invalid solar system/campaign - " (`|GetEnumeratorNameAsString` (`local.Campaign`)))))))