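; Space tutorial component that sequences the steps from Intro through Escape, extending a parent tutorial class.
; Loads each step's row from DT_TutorialSteps by enum name, then dispatches step-start and dialogue-finished handlers by current step.
; Navigate spawns destination markers in the starting solar system and ends once all are reached.
; Intro, Capture and Destroy end when dialogue finishes; the other start and dialogue handlers are empty stubs.
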(fn `CallStepOutOfOrder`
  (params (Step :type "/Game/GlobalEnums/E_TutorialSteps Enum" :default "NewEnumerator0"))
  (`self.LoadStepData` "NewEnumerator0")
  (`self.RunStepFirstTime`))

(fn `DialogueFinishedCapture`
  (`self.EndStep`))

(fn `DialogueFinishedCombat`)

(fn `DialogueFinishedDestroy`
  (`self.EndStep`))

(fn `DialogueFinishedEscape`)

(fn `DialogueFinishedIntercept`)

(fn `DialogueFinishedIntro`
  (`self.EndStep`))

(fn `DialogueFinishedNavigate`)

(fn `DialogueFinishedRetreat`)

(fn `LoadStepData`
  (params (Step :type "/Game/GlobalEnums/E_TutorialSteps Enum" :default "NewEnumerator0"))
  (bind _output_get (set `self.CurrentStep` Step))
  (bind _returnvalue (`|GetEnumeratorNameAsString` _output_get))
  (bind _returnvalue_2 (`|GetDataTableRow` "/Game/DataTables/DT_TutorialSteps.DT_TutorialSteps" (`KismetStringLibrary.Conv_StringToName` _returnvalue))
    (:`then`
      (set `self.StepTutorialData` _returnvalue_2))
    (:`RowNotFound`
      (set `self.StepTutorialData` (struct))
      (`/JGGErrorAndTesting/FunctionLibraries/FL_Error.PrintMessage` null "NewEnumerator2" (`KismetStringLibrary.Concat_StrStr` _returnvalue " - Objective Has No Data")))))

(fn `OnAllDialogueFinished`
  (`parent.OnAllDialogueFinished`)
  (switch `/Game/GlobalEnums/E_TutorialSteps` (`self.CurrentStep`)
    (:`NewEnumerator1`
      (`self.DialogueFinishedIntro`))
    (:`NewEnumerator2`
      (`self.DialogueFinishedNavigate`))
    (:`NewEnumerator3`
      (`self.DialogueFinishedIntercept`))
    (:`NewEnumerator4`
      (`self.DialogueFinishedCombat`))
    (:`NewEnumerator9`
      (`self.DialogueFinishedRetreat`))
    (:`NewEnumerator7`
      (`self.DialogueFinishedCapture`))
    (:`NewEnumerator8`
      (`self.DialogueFinishedDestroy`))
    (:`NewEnumerator5`
      (`self.DialogueFinishedEscape`))))

(fn `OnNavigationPointReached`
  (bind _result (`/Engine/EditorBlueprintResources/StandardMacros.IncrementInt` (`self.NumNavigationPointsFound`))
    (:`  `
      (if (>= _result (`KismetArrayLibrary.Array_Length` (`self.NavigationPoints`)))
        (`self.EndStep`)))))

(fn `RunStep`
  (params (bFirstTime :type Boolean))
  (`parent.RunStep` bFirstTime)
  (switch `/Game/GlobalEnums/E_TutorialSteps` (`self.CurrentStep`)
    (:`NewEnumerator1`
      (`self.StartIntro`))
    (:`NewEnumerator2`
      (`self.StartNavigate`))
    (:`NewEnumerator3`
      (`self.StartIntercept`))
    (:`NewEnumerator4`
      (`self.StartCombat`))
    (:`NewEnumerator9`
      (`self.StartRetreat`))
    (:`NewEnumerator7`
      (`self.StartCapture`))
    (:`NewEnumerator8`
      (`self.StartDestroy`))
    (:`NewEnumerator5`
      (`self.StartEscape`))))

(fn `StartCapture`)

(fn `StartCombat`)

(fn `StartDestroy`)

(fn `StartEscape`)

(fn `StartIntercept`)

(fn `StartIntro`)

(fn `StartNavigate`
  (locals (System :type "/Game/Actors/BP_SolarSystem Object Reference"))
  (bind _system (`local.System`))
  (bind (_value _returnvalue) (`BlueprintMapLibrary.Map_Find` (`/Game/ActorComponents/BP_CampaignManager.SolarSystems` (`self.CampaignManager`)) (`self.StartingSystem`)))
  (if _returnvalue
    (set `local.System` _value)
    (set `self.NumNavigationPointsFound` 0)
    (for _array_element (`self.NavigationPoints`)
      (bind _returnvalue_2 (`|AddComponentByClass` _system "/Game/SceneComponents/BP_TutorialDestination.BP_TutorialDestination_C" false (`/JGGUniversalFunctionsAndMacros/FunctionLibraries/FL_Transformation.Relative2DToWorldTransform3D` (0.0 0.0 0.0) _array_element (`.Radius_58_FF405E09454FF9C40FC9808B1FC38F34` (break `/Game/Structs/S_SolarSystemData` (`/Game/Actors/BP_SolarSystem.SolarSystemData` (`local.System`)))) (/ (defaults `/Game/SceneComponents/BP_TutorialDestination` "/Game/SceneComponents/BP_TutorialDestination.BP_TutorialDestination_C") 50.0)) _system))
      (`KismetArrayLibrary.Array_Add` (`/Game/Actors/BP_SolarSystem.Clickables` (`local.System`)) _returnvalue_2)
      (add `/Game/SceneComponents/BP_TutorialDestination.PlayerReached` _returnvalue_2 (`|CreateDelegate` :!event `OnNavigationPointReached`)))))

(fn `StartRetreat`)

(fn `UpdateStepEnum`
  (`parent.UpdateStepEnum`)
  (`self.LoadStepData` (`|GetArrayItem` (`self.Steps`) (`self.GetCurrentStepIndex`))))